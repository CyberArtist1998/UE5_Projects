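; AI controller for enemy warships that runs the BT_EnemyWarship behavior tree and tracks the player by sight.
; Perception updates go to HandleSightSense, which sets the TargetPawn blackboard key to the player pawn when seen and clears it when sight is lost.
; A helper caches the player pawn cast to BP_WarshipMainPlayer, but its delayed retry loop in the event graph never runs.
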(event OnTargetPerceptionUpdated(AIPerception)
  (params (Actor :type Actor%20Object%20Reference) (Stimulus :type AI%20Stimulus%20Structure))
  (if true
    (CallFunction|HandleSightSense Actor Stimulus)
    (else
      (Development|PrintString "Sense is not available becaause cast to playerPawn is still not set" true true "(R=0.016631,G=0.000000,B=0.742000,A=1.000000)" 0.0))))

(event EventBeginPlay
  (AI|RunBehaviorTree "/Game/1_MyWorkingSpace/BluePrint/AI/BT_EnemyWarship.BT_EnemyWarship"))

(fn ConstructionScript)

(fn HandleSightSense
  (params (Actor :type Actor%20Object%20Reference) (Stimulats :type AI%20Stimulus%20Structure))
  (bind _bsuccessfullysensed (Utilities|Struct|BreakAIStimulus Stimulats))
  (bind _returnvalue (Class|AIPerceptionSystem|GetSenseClassforStimulus Stimulats))
  (if (== _returnvalue "/Script/AIModule.AISense_Sight")
    (if (== Actor (Game|Player|GetPlayerPawn 0))
      (AI|Components|Blackboard|SetValueasObject (Variables|Default|GetBlackboard) (Utilities|Name|MakeLiteralName "TargetPawn") (Utilities|SelectObject (Game|Player|GetPlayerPawn 0) 0 _bsuccessfullysensed))
      (if _bsuccessfullysensed
        _)
      (else
        (return)))
    (else
      (return))))

(fn GetPlayerPawn
  (Utilities|IsValid (Variables|Default|GetAs%20BP%20Warship%20Main%20Player)
    (:Is%20Valid
      _)
    (:Is%20Not%20Valid
      (bind _asbp_warship_main_player (Utilities|Casting|CastToBP_WarshipMainPlayer (Game|Player|GetPlayerPawn 0))
        (:then
          (Variables|Default|SetAs%20BP%20Warship%20Main%20Player _asbp_warship_main_player))
        (:CastFailed
          (return (Variables|Default|GetAs%20BP%20Warship%20Main%20Player))))))
  (return (Variables|Default|GetAs%20BP%20Warship%20Main%20Player)))