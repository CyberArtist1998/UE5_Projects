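; Behavior tree task that sends the controlled pawn to a random reachable navmesh point within Radius of its location.
; AI MoveTo uses AcceptanceRadius and finishes the task as success or failure when the move ends.
; Its immediate output branches on the movement result to draw a debug sphere and print a location, or print an error.
; The random point is re-rolled for each debug call, so shown locations can differ from the destination.
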(event EventReceiveExecuteAI
  (params (OwnerController :type AI%20Controller%20Object%20Reference) (ControlledPawn :type Pawn%20Object%20Reference))
  (bind _returnvalue (Transformation|GetActorLocation ControlledPawn))
  (bind _radius (Variables|Default|GetRadius))
  (bind _randomlocation (AI|Navigation|GetRandomReachablePointinRadius _returnvalue _radius 0 0))
  (bind _movementresult (AI|AIMoveTo ControlledPawn _randomlocation 0 (Variables|Default|GetAcceptance%20Radius) false)
    (:then
      (if (Utilities|Select :Index _movementresult :Success true :Blocked true :OffPath true :Aborted false :Invalid false)
        (Rendering|Debug|DrawDebugSphere _randomlocation 2.5e+03 25 "(R=0.000000,G=1.000000,B=0.027720,A=1.000000)" 1.0)
        (Development|PrintString (Utilities|String|Append "Random Location to Move to :" (Utilities|String|ToString(Vector) _randomlocation)) true true "(R=0.000000,G=1.000000,B=0.027720,A=1.000000)")
        (else
          (Development|PrintString "Random Location to Move to is ABOARTED or UNVALID" true true "(R=1.000000,G=0.000000,B=0.013299,A=1.000000)" 0.0))))
    (:OnSuccess
      (AI|BehaviorTree|FinishExecute true))
    (:OnFail
      (AI|BehaviorTree|FinishExecute false))))