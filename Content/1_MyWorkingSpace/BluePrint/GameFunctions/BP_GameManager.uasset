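; Game manager Blueprint that tracks enemy small boats and warships in the warship game mode.
; On BeginPlay it caches the BP_WarshipMainGameMode reference.
; EnemyCounter gathers both AI classes tagged "Enemy", totals them, subtracts one, and calls the game mode's Victory when none remain.
; AddOrRemoveEnemy only increments the selected type's count, updates the total for warships and boats, and prints debug messages.
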(event EventBeginPlay
  (CallFunction|GetGameMode))

(fn ConstructionScript)

(fn GetGameMode
  (Utilities|IsValid (Variables|Default|GetGame%20Mode)
    (:Is%20Valid
      _)
    (:Is%20Not%20Valid
      (bind _asbp_warship_main_game_mode (Utilities|Casting|CastToBP_WarshipMainGameMode (Game|GetGameMode))
        (:then
          (bind _output_get (Variables|Default|SetGame%20Mode _asbp_warship_main_game_mode)))
        (:CastFailed
          (return 0)))))
  (return _output_get))

(fn EnemyCounter
  (bind _outactors (Actor|GetAllActorsOfClasswithTag "/Game/1_MyWorkingSpace/BluePrint/Characters/BP_MasterAI-SmallBouts.BP_MasterAI-SmallBouts_C" "Enemy"))
  (bind _output_get (Variables|Default|SetEnemies%20-%20SmallBouts _outactors))
  (Variables|Default|SetEnemies_Number%20-%20SmallBouat (Utilities|Array|Length _output_get))
  (for _array_element _output_get
    (Utilities|Array|Add (Variables|Default|GetEnemies%20-%20Total) _array_element))
  (bind _outactors_2 (Actor|GetAllActorsOfClasswithTag "/Game/1_MyWorkingSpace/BluePrint/Characters/BP_MasterAI-SkInRot.BP_MasterAI-SkInRot_C" "Enemy"))
  (bind _output_get_2 (Variables|Default|SetEnemies%20-%20Warships _outactors_2))
  (Variables|Default|SetEnemies_Number%20-%20Warship (Utilities|Array|Length _output_get_2))
  (for _array_element_2 _output_get_2
    (Utilities|Array|Add (Variables|Default|GetEnemies%20-%20Total) _array_element_2))
  (bind _output_get_3 (Variables|Default|SetEnemies_Number%20-%20Total (+ (Variables|Default|GetEnemies_Number%20-%20Warship) (Variables|Default|GetEnemies_Number%20-%20SmallBouat))))
  (if true
    (Development|PrintString (Utilities|String|Append "Counting Done." (Utilities|String|ToString(Integer) _output_get_3))))
  ;[0.15 0.15 0.15 0.5] Comment
  (Math|Integer|DecrementInt (Variables|Default|GetEnemies_Number%20-%20Total)
    (:%20%20
      (if (> (Variables|Default|GetEnemies_Number%20-%20Total) 0)
        (return (Variables|Default|GetEnemies_Number%20-%20SmallBouat) (Variables|Default|GetEnemies_Number%20-%20Warship) (Variables|Default|GetEnemies_Number%20-%20Total))
        (else
          (Default|Victory (Variables|Default|GetGame%20Mode)))))))

(fn AddorRemoveEnemy
  (params (Selection :type E_ActorsName%20Enum :default "NewEnumerator3"))
  (switch Utilities|FlowControl|Switch|SwitchonE_ActorsName Selection
    (:NewEnumerator0
      (bind _result (Math|Integer|IncrementInt (Variables|Default|GetEnemies_Number%20-%20Warship))
        (:%20%20
          (bind _output_get (Variables|Default|SetEnemies_Number%20-%20Warship _result))
          (if true ; Debug
            (|Debugger-Warship_2 _output_get)))))
    (:NewEnumerator1
      (bind _result_2 (Math|Integer|IncrementInt (Variables|Default|GetEnemies_Number%20-%20SmallBouat))
        (:%20%20
          (bind _output_get_2 (Variables|Default|SetEnemies_Number%20-%20SmallBouat _result_2))
          (if true ; Debug
            (|Debugger-SmallBout_2 _output_get_2))))))
  (Variables|Default|SetEnemies_Number%20-%20Total (+ (Variables|Default|GetEnemies_Number%20-%20Warship) (Variables|Default|GetEnemies_Number%20-%20SmallBouat))))