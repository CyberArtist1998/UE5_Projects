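; Warship game mode that starts play and handles pause, victory, game over and return to the main menu.
; On BeginPlay it caches controller, HUD and camera references, spawns the player warship with a retry loop, possesses it and enables touch, with a camera intro and delayed outro.
; Bound dispatchers drive game-state changes through HUD layouts or level loads.
; A bound kill switch applies lethal damage to all listed enemy boats and warships.
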(event Custom|Initial%20Protocol%20Phase%201
  ;[0 0 0 0.5] Initial P:rotocols - Recived trigger from 'menuV2' to start the actual game
  (bind _output_get (|SpawnPlayerActor_2))
  (|SetPlayerasWarshipActor_2 _output_get)
  (Default|ChangeUILayout (Variables|Default|GetAs%20BP%20HUD_0) "NewEnumerator0")
  (Default|CameraAnimation-Intro (Variables|Default|GetCamera%20Animation))
  (Pawn|Possess (Game|GetPlayerController 0) (Variables|Game|GetGame%20-%20PlayerWarship))
  (Default|CallEDWarshipIsActivated (Variables|Default|GetAs%20BP%20WS%20Player%20Controler_0)) ; REciver is in PC ( Player Controller )
  (Variables|/Game/1_MyWorkingSpace/BluePrint/GameFunctions/BP_WarshipPlayerControler.BP_WarshipPlayerControler_C|SetTouch%20Is%20Allowed? (Variables|Default|GetAs%20BP%20WS%20Player%20Controler_0) true))

(event EventBeginPlay
  (Utilities|FlowControl|Sequence
    (:then_0
      (CallFunction|GetPC)
      (CallFunction|GetHUD)
      (CallFunction|GetCameraAnimation)
      (CallFunction|InitialProtocolPhase1))
    (:then_1
      (|BindEvent-GameStates))
    (:then_2
      (|KillSwitch))
    (:then_3
      (Utilities|FlowControl|Delay 6.0)
      (Default|CameraAnimation-Outro (Variables|Default|GetCamera%20Animation)))))

(fn ConstructionScript)

(fn GetHUD
  (Utilities|IsValid (Variables|Default|GetAs%20BP%20HUD_0)
    (:Is%20Valid
      _)
    (:Is%20Not%20Valid
      (bind _asbp_warship_hud (Utilities|Casting|CastToBP_WarshipHUD (HUD|GetHUD (Game|GetPlayerController 0)))
        (:then
          (Variables|Default|SetAs%20BP%20HUD_0 _asbp_warship_hud))
        (:CastFailed
          (Development|PrintString "Cast is Failed to HUD" true true "(R=1.000000,G=0.000000,B=0.013299,A=1.000000)")
          (return (Variables|Default|GetAs%20BP%20HUD_0))))))
  (return (Variables|Default|GetAs%20BP%20HUD_0)))

(fn GetPC
  (Utilities|IsValid (Variables|Default|GetAs%20BP%20WS%20Player%20Controler_0)
    (:Is%20Valid
      _)
    (:Is%20Not%20Valid
      (bind _asbp_warship_player_controler (Utilities|Casting|CastToBP_WarshipPlayerControler (Game|GetPlayerController 0))
        (:then
          (Variables|Default|SetAs%20BP%20WS%20Player%20Controler_0 _asbp_warship_player_controler))
        (:CastFailed
          (Development|PrintString "Cast to WS PlayerController Failed" true true "(R=1.000000,G=0.000000,B=0.013299,A=1.000000)")
          (return (Variables|Default|GetAs%20BP%20WS%20Player%20Controler_0))))))
  (return (Variables|Default|GetAs%20BP%20WS%20Player%20Controler_0)))

(fn GetGameManager
  (bind _returnvalue (Actor|GetActorOfClass "/Game/1_MyWorkingSpace/BluePrint/GameFunctions/BP_GameManager.BP_GameManager_C"))
  (Utilities|IsValid (Variables|Default|GetAs%20BP%20Game%20Manager)
    (:Is%20Valid
      _)
    (:Is%20Not%20Valid
      (bind _asbp_game_manager (Utilities|Casting|CastToBP_GameManager _returnvalue)
        (:then
          (bind _output_get (Variables|Default|SetAs%20BP%20Game%20Manager _asbp_game_manager)))
        (:CastFailed
          (return 0)))))
  (return _output_get))

(fn GetCameraAnimation
  (bind _returnvalue (Actor|GetActorOfClass "/Game/1_MyWorkingSpace/BluePrint/GameFunctions/BP_CameraAnimation.BP_CameraAnimation_C"))
  (bind _output_get (Variables|Default|SetCamera%20Animation _returnvalue))
  (return _output_get))

(event Custom|Victory
  ;[0.01706 0.4941 0] BackToMainMenu
  (Default|ChangeUILayout (Variables|Default|GetAs%20BP%20HUD_0) "NewEnumerator6"))

(event Custom|GameOver!
  ;[1 0 0.0133] Game Over!
  (Input|SetInputModeUIOnly (Game|GetPlayerController 0) 0 "DoNotLock" false)
  (Viewport|RemoveAllWidgets)
  (bind _returnvalue (UserInterface|CreateWidget "/Game/1_MyWorkingSpace/UI/V2/23Died_WB.23Died_WB_C"))
  (UserInterface|Viewport|AddtoViewport _returnvalue 0)
  (Utilities|FlowControl|Delay 2.0)
  (Game|OpenLevel(byName) "Lvl_X_TestField"))

(event Custom|BackToMainMenu
  ;[0.395 0.4941 0] BackToMainMenu
  (Input|SetInputModeUIOnly (Game|GetPlayerController 0) 0 "DoNotLock" false)
  (Viewport|RemoveAllWidgets)
  (Game|OpenLevel(byName) "L_MainMenu"))

(event Custom|Puase/UnPause
  (bind _as_bp_hud_0 (Variables|Default|GetAs%20BP%20HUD_0))
  ;[1 0.4956 0] Puase/UnPause
  (Utilities|FlowControl|FlipFlop
    (:A
      (Default|ChangeUILayout _as_bp_hud_0 "NewEnumerator4")
      (Game|SetGamePaused true))
    (:B
      (Default|ChangeUILayout _as_bp_hud_0 "NewEnumerator0")
      (Game|SetGamePaused false))))

(event Custom|ED_GameRestart_Event
  ;[0.15 0.15 0.15 0.5] Game state
  (CallFunction|BacktoMainMenu))

(event Custom|ED_Victory_Event
  ;[0.15 0.15 0.15 0.5] Game state
  (CallFunction|Victory))

(event Custom|ED_GameStarted_Event
  ;[0.15 0.15 0.15 0.5] Game state
  (CallFunction|InitialProtocolPhase1))

(event Custom|ED_GamePause_Event
  ;[0.15 0.15 0.15 0.5] Game state
  (CallFunction|Puase/UnPause))

(event Custom|ED_GameOver!_Event
  ;[0.15 0.15 0.15 0.5] Game state
  (CallFunction|GameOver!))

(event Custom|KillThemALL
  ;[0.15 0.15 0.15 0.5] Kill Switch
  (for _array_element (Variables|Default|GetEnemies%20-%20SmallBouts)
    (Game|Damage|ApplyDamage _array_element 1e+04 0 0 "/Script/Engine.DamageType"))
  (for _array_element_2 (Variables|Default|GetEnemies%20-%20Warships)
    (Game|Damage|ApplyDamage _array_element_2 1e+04 0 0 "/Script/Engine.DamageType"))
  (Development|PrintString "All Enemies are killed"))

(fn GetPatrolPath
  (return 0))