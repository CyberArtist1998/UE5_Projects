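; Player controller for the turret test field that possesses the test turret pawn on BeginPlay and aims it by touch drag.
; Each touch move turns the scaled, clamped delta from the previous position into controller yaw and pitch input.
; Interface events forward health to the master UI widget and bullet firing to the warship player.
; Also holds debug key toggles and unfinished or uncalled helpers for widgets, HUD lookup and homing-missile targeting.
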(event EventBPIWFShootingBullets
  ;[1 1 1] BPI
  (Default|FirePattern (Variables|Default|GetAs%20BP%20Warship%20Main%20Player_0)))

(event EventBeginPlay
  (Utilities|FlowControl|Sequence
    (:then_0
      (bind _as_bp_warship_main_player_test (Getter|GetTurretTestChar))
      (Utilities|IsValid _as_bp_warship_main_player_test
        (:Is%20Valid
          (Pawn|Possess _as_bp_warship_main_player_test)
          (Variables|Default|SetTouch%20Is%20Allowed? true))))))

(event EventBPIWFHealth
  (params (BPI_WF%20Heaalth%20value%20input :type Integer))
  ;[1 1 1] BPI
  (Default|BPIWFHealth (Variables|UI|GetWB%20UI%20Master%20) BPI_WF%20Heaalth%20value%20input))

(event Input|KeyboardEvents|D
  (params (Key :type Key%20Structure))
  ;[0.15 0.15 0.15 0.5] Debugger switch
  (:Pressed
    (Utilities|FlowControl|FlipFlop
      (:A
        (Variables|Default|SetDebugger true))
      (:B
        (Variables|Default|SetDebugger false)))))

(event Input|TouchEvents|InputTouch
  (params (Location :type Vector) (FingerIndex :type ETouchIndex%20Enum))
  (bind (_x _y) (Math|Vector|BreakVector Location))
  ;[1 0.7876 0.5244] Touch Screen Camera Look
  ;
  ; NOTE:
  ; For time being , the Input Method is set throught BP_HUD. Setting input method to UI Only cause the InputTouch to NOT recived anyhing
  (:Pressed
    (if (Variables|Default|GetTouch%20Is%20Allowed?) :!label _label
      (Variables|Default|SetStart%20Postion (Math|Vector2D|MakeVector2D _x _y) :!label _label_2)))
  (:Released
    (goto _label))
  (:Moved
    (if (Variables|Default|GetTouch%20Is%20Allowed?)
      (TouchandCamera|Touch-UpdatePosition (Math|Vector2D|MakeVector2D _x _y) (Variables|UI|GetUI%20Mode))
      (goto _label_2))))

(fn ConstructionScript)

(fn ToggleWidget
  (params (Widget%20to%20Focuse :type User%20Widget%20Object%20Reference))
  (Utilities|IsValid Widget%20to%20Focuse
    (:Is%20Valid
      (Variables|/Script/UMG.Widget|SetVisibility Widget%20to%20Focuse "Collapsed")
      (return))
    (:Is%20Not%20Valid
      (Development|PrintString "Previouse Widget is not valid")
      (return))))

(fn FocuseWidget
  (Widget|SetVisibility (Variables|UI|GetWidget%20To%20Focus) "SelfHitTestInvisible"))

(fn GetLowHealthWb)

(fn FindHomingTargetMissile
  (bind _homingtarget (LocalVariables|GetHomingTarget))
  (bind _returnvalue (Actor|GetComponentbyClass _homingtarget "/Script/Engine.SceneComponent"))
  (bind _outactors (Actor|GetAllActorsOfClasswithTag "/Script/Engine.Actor" (Variables|Enemy|GetEnemy%20-%20Tag%20name)))
  (bind _output_get (LocalVariables|SetNewVar_0 (Utilities|Array|IsNotEmpty _outactors)))
  (bind _output_get_2 (Variables|Enemy|SetEnemy%20-%20All _outactors))
  (if _output_get
    (for _array_element _output_get_2
      (if true ; Missile In range?
        (Variables|Enemy|SetEnemy%20-%20single%20with%20tag _array_element)
        (LocalVariables|SetDistanceToTarget (Math|Vector|VectorLength (- (Transformation|GetActorLocation _array_element) (Transformation|GetActorLocation))))))
    (Utilities|IsValid _returnvalue
      (:Is%20Valid
        (return _returnvalue))
      (:Is%20Not%20Valid
        (Development|PrintString "There is no SC with Homing Tag in map")))
    (else
      (Development|PrintString "Could not find any target for missile to hit"))))

(fn Touch-UpdatePosition
  (params (Update%20psotion :type Vector%202D%20Structure) (UI%20Mode :type E_SwitchForTargetRecievInputTouch%20Enum :default "NewEnumerator0"))
  (bind _turretpawn_test (Variables|Default|GetTurretPawn_Test))
  (bind _start_postion (Variables|Default|GetStart%20Postion))
  (bind _touchsensevity (Variables|Touch|GetTouchSensevity))
  (bind _returnvalue (- Update%20psotion _start_postion))
  (bind _returnvalue_2 (* _returnvalue _touchsensevity))
  ;[1 1 1] Update Postion
  (|Debug-InputPostion (.x _returnvalue_2) (.y _returnvalue_2))
  (LocalVariables|SetClamp%20Float%20X (Math|Float|Clamp(Float) (.x _returnvalue_2) -1.0))
  (LocalVariables|SetClamp%20Float%20Y (Math|Float|Clamp(Float) (.y _returnvalue_2) -1.0))
  (Utilities|IsValid _turretpawn_test
    (:Is%20Valid
      (Pawn|Input|AddControllerYawInput _turretpawn_test (LocalVariables|GetClamp%20Float%20X))
      (Pawn|Input|AddControllerPitchInput _turretpawn_test (LocalVariables|GetClamp%20Float%20Y)))
    (:Is%20Not%20Valid
      (Development|PrintString "Touch Target pawn is not Valid"))))

(fn GetMasterUI
  (bind _returnvalue (Game|ConstructObjectfromClass "/Game/1_MyWorkingSpace/UI/WB_MasterUI.WB_MasterUI_C"))
  (bind _output_get (Variables|UI|SetWB%20UI%20Master%20 _returnvalue))
  (UserInterface|Viewport|AddtoViewport _output_get 0))

(fn GetTurret76mm
  (bind _returnvalue (Actor|GetActorOfClass "/Game/1_MyWorkingSpace/BluePrint/Weapons/BP_Turret_76mm.BP_Turret_76mm_C"))
  (Variables|Default|SetTurret%2076mm _returnvalue))

(fn GetTurretTestChar
  (Utilities|IsValid (Variables|Default|GetAs%20BP%20Lvl%20X%20Turret%20Test%20Field%20Game%20Mode)
    (:Is%20Valid
      _)
    (:Is%20Not%20Valid
      (bind _asbp_turret_pawn_test (Utilities|Casting|CastToBP_TurretPawn_Test (Game|Player|GetPlayerPawn 0))
        (:then
          (Variables|Default|SetTurretPawn_Test _asbp_turret_pawn_test))
        (:CastFailed
          (return (Variables|Default|GetTurretPawn_Test))))))
  (return (Variables|Default|GetTurretPawn_Test)))

(event Custom|Green%20Debuger
  (params (Location%20/%20 :type String) (Message%20/ :type String))
  ;[0 0.5781 1] Debuger
  ;;[0.1 1 0] Green Debugger
  (if (Variables|Temp|GetDebuger%20Switch)
    (Development|PrintString (Utilities|String|Append Location%20/%20 Message%20/) true true "(R=0.100000,G=1.000000,B=0.000000,A=1.000000)" 0.2 "")))

(event Custom|Red%20Debuger
  (params (Location%20/%20 :type String) (Message%20/ :type String))
  ;[0 0.5781 1] Debuger
  ;;[1 0 0.005087] Red Debugger
  (if (Variables|Temp|GetDebuger%20Switch)
    (Development|PrintString (Utilities|String|Append Location%20/%20 Message%20/) true true "(R=1.000000,G=0.000000,B=0.005088,A=1.000000)")))

(event Input|KeyboardEvents|P
  (params (Key :type Key%20Structure))
  ;[0 0.5781 1] Debuger
  ;;[0.1 1 0] Green Debugger
  (:Pressed
    (if (Variables|Temp|GetDebuger%20Switch)
      (Development|PrintString (Utilities|String|Append (stale Custom|Green%20Debuger Location%20/%20) (stale Custom|Green%20Debuger Message%20/)) true true "(R=0.100000,G=1.000000,B=0.000000,A=1.000000)" 0.2 ""))))

(event Input|KeyboardEvents|P
  (params (Key :type Key%20Structure))
  ;[0 0.5781 1] Debuger
  ;;[1 0 0.005087] Red Debugger
  (:Pressed
    (Utilities|FlowControl|FlipFlop
      (:A
        (Variables|Temp|SetDebuger%20Switch true))
      (:B
        (Variables|Temp|SetDebuger%20Switch false)))
    (if (Variables|Temp|GetDebuger%20Switch)
      (Development|PrintString (Utilities|String|Append (stale Custom|Red%20Debuger Location%20/%20) (stale Custom|Red%20Debuger Message%20/)) true true "(R=1.000000,G=0.000000,B=0.005088,A=1.000000)"))))

(fn GetPatrolPath
  (return 0))