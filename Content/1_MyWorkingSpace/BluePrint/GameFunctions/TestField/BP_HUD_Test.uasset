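; Test HUD Blueprint that creates the game's UI screens at BeginPlay and switches between them by UI mode.
; It adds every widget to the viewport and an array, collapses all, then calls ChangeUILayout.
; Player, pause, death, victory and main menu modes collapse other widgets via a temporary array and set cursor, focus and input mode.
; Submenu modes only show their widget and trim that array, while Clean/Animation collapses its contents.
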(event Custom|Change%20UI%20Layout
  (params (UI%20Mode :type E_Switch_Widgets%20Enum :default "NewEnumerator1"))
  (bind _returnvalue (Game|GetPlayerController 0))
  (bind _mm_mainmenu (Variables|Widgets|GetMM_MainMenu))
  (bind _pause_menu (Variables|Widgets|GetPause%20Menu))
  (bind _player_ui (Variables|Widgets|GetPlayer%20UI))
  (bind _death_ui (Variables|Widgets|GetDeath%20UI))
  (bind _vectory_ui (Variables|Widgets|GetVectory%20UI))
  (bind _output_get (Variables|Default|SetUI%20Mode UI%20Mode))
  (switch Utilities|FlowControl|Switch|SwitchonE_Switch_Widgets _output_get
    (:NewEnumerator4
      (bind _output_get_2 (Variables|Default|SetWidget%20to%20Focuse _pause_menu))
      (Variables|Default|SetUI%20Only%20or%20GameandUI true) ; True > UI Only\nFalse > Game and UI
      (Widget|SetVisibility _output_get_2 "Visible")
      (Utilities|Array|RemoveItem (Variables|Default|GetAll%20WIdgets%20Temp) _pause_menu)
      ;[1 0 0.0133] Offline Widgets
      (for _array_element (Variables|Default|GetAll%20WIdgets%20Temp) :!label _label
        (Widget|SetVisibility _array_element "Collapsed"))
      (Variables|/Script/Engine.PlayerController|SetbShowMouseCursor (Game|GetPlayerController 0) true)
      (Variables|Default|SetAll%20WIdgets%20Temp (Variables|Default|GetAll%20WIdgets))
      (if (Variables|Default|GetUI%20Only%20or%20GameandUI) ; True > UI Only\nFalse > Game and UI
        (Input|SetInputModeUIOnly _returnvalue (Variables|Default|GetWidget%20to%20Focuse) "DoNotLock" false)
        (else
          (Input|SetInputModeGameandUI _returnvalue (Variables|Default|GetWidget%20to%20Focuse) "DoNotLock" false false))))
    (:NewEnumerator0
      (bind _output_get_3 (Variables|Default|SetWidget%20to%20Focuse _player_ui))
      (Variables|Default|SetUI%20Only%20or%20GameandUI false) ; True > UI Only\nFalse > Game and UI
      (Widget|SetVisibility _output_get_3 "Visible")
      (Utilities|Array|RemoveItem (Variables|Default|GetAll%20WIdgets%20Temp) _player_ui)
      (goto _label))
    (:NewEnumerator5
      (bind _output_get_4 (Variables|Default|SetWidget%20to%20Focuse _death_ui))
      (Variables|Default|SetUI%20Only%20or%20GameandUI true) ; True > UI Only\nFalse > Game and UI
      (Widget|SetVisibility _output_get_4 "Visible")
      (Utilities|Array|RemoveItem (Variables|Default|GetAll%20WIdgets%20Temp) _death_ui)
      (goto _label))
    (:NewEnumerator6
      (bind _output_get_5 (Variables|Default|SetWidget%20to%20Focuse _vectory_ui))
      (Variables|Default|SetUI%20Only%20or%20GameandUI true) ; True > UI Only\nFalse > Game and UI
      (Widget|SetVisibility _output_get_5 "Visible")
      (Utilities|Array|RemoveItem (Variables|Default|GetAll%20WIdgets%20Temp) _vectory_ui)
      (goto _label))
    (:NewEnumerator1
      ;[0.15 0.15 0.15 0.5] Main Menu
      (bind _output_get_6 (Variables|Default|SetWidget%20to%20Focuse _mm_mainmenu))
      (Variables|Default|SetUI%20Only%20or%20GameandUI true) ; True > UI Only\nFalse > Game and UI
      (Widget|SetVisibility _output_get_6 "Visible")
      (Utilities|Array|RemoveItem (Variables|Default|GetAll%20WIdgets%20Temp) _mm_mainmenu)
      (goto _label))
    (:NewEnumerator7
      ;[0.15 0.15 0.15 0.5] Shop
      (bind _output_get_7 (Variables|Default|SetWidget%20to%20Focuse (Variables|Widgets|GetMM_Shop)))
      (Variables|Default|SetUI%20Only%20or%20GameandUI true) ; True > UI Only\nFalse > Game and UI
      (Widget|SetVisibility _output_get_7 "Visible")
      (Utilities|Array|RemoveItem (Variables|Default|GetAll%20WIdgets%20Temp) _output_get_7)
      (Utilities|Array|RemoveItem (Variables|Default|GetAll%20WIdgets%20Temp) (Variables|Widgets|GetMM_MainMenu) :!label _label_2) ; Keep the MainMenu UI in place
    )
    (:NewEnumerator8
      ;[0.15 0.15 0.15 0.5] Harbore
      (bind _output_get_8 (Variables|Default|SetWidget%20to%20Focuse (Variables|Widgets|GetMM_Harbore)))
      (Variables|Default|SetUI%20Only%20or%20GameandUI true) ; True > UI Only\nFalse > Game and UI
      (Widget|SetVisibility _output_get_8 "Visible")
      (Utilities|Array|RemoveItem (Variables|Default|GetAll%20WIdgets%20Temp) _output_get_8)
      (goto _label_2))
    (:NewEnumerator9
      ;[0.15 0.15 0.15 0.5] Setting
      (bind _output_get_9 (Variables|Default|SetWidget%20to%20Focuse (Variables|Widgets|GetMM_Setting)))
      (Variables|Default|SetUI%20Only%20or%20GameandUI true) ; True > UI Only\nFalse > Game and UI
      (Widget|SetVisibility _output_get_9 "Visible")
      (Utilities|Array|RemoveItem (Variables|Default|GetAll%20WIdgets%20Temp) _output_get_9)
      (goto _label_2))
    (:NewEnumerator10
      ;[0.15 0.15 0.15 0.5] Story Map > MissionExplanation
      (bind _output_get_10 (Variables|Default|SetWidget%20to%20Focuse (Variables|Widgets|GetMM_StoryMap)))
      (Variables|Default|SetUI%20Only%20or%20GameandUI true) ; True > UI Only\nFalse > Game and UI
      (Widget|SetVisibility _output_get_10 "Visible")
      (Utilities|Array|RemoveItem (Variables|Default|GetAll%20WIdgets%20Temp) _output_get_10)
      (goto _label_2))
    (:NewEnumerator12
      (bind _output_get_11 (Variables|Default|SetWidget%20to%20Focuse (Variables|Widgets|GetMM_Setting)))
      (Variables|Default|SetUI%20Only%20or%20GameandUI true) ; True > UI Only\nFalse > Game and UI
      (Widget|SetVisibility _output_get_11 "Visible")
      (Utilities|Array|RemoveItem (Variables|Default|GetAll%20WIdgets%20Temp) _output_get_11)
      (goto _label_2))
    (:NewEnumerator3
      ;[0.15 0.15 0.15 0.5] GameModeSelection > StoryMap
      (Variables|Default|SetUI%20Only%20or%20GameandUI true) ; True > UI Only\nFalse > Game and UI
      (for _array_element_2 (Variables|Default|GetAll%20WIdgets%20Temp)
        (Widget|SetVisibility _array_element_2 "Collapsed")))))

(event EventBeginPlay
  (bind _all_widgets (Variables|Default|GetAll%20WIdgets))
  (Utilities|FlowControl|Sequence ; There are some better ways to create widgets but one thing to notice:\nfor example If we start to add them to an array, then add to view port,\nIn what order they are created ?
    (:then_0
      (bind _returnvalue (UserInterface|CreateWidget "/Game/1_MyWorkingSpace/UI/WB_MasterUI_TurretPawnTest.WB_MasterUI_TurretPawnTest_C"))
      (Utilities|IsValid _returnvalue
        (:Is%20Valid
          (bind _output_get (Variables|Widgets|SetPlayer%20UI _returnvalue))
          (UserInterface|Viewport|AddtoViewport _output_get 0)
          (Utilities|Array|Add (Variables|Default|GetAll%20WIdgets) _output_get))))
    (:then_1
      (bind _returnvalue_2 (UserInterface|CreateWidget "/Game/1_MyWorkingSpace/UI/V2/21Pause_WB.21Pause_WB_C"))
      (Utilities|IsValid _returnvalue_2
        (:Is%20Valid
          (bind _output_get_2 (Variables|Widgets|SetPause%20Menu _returnvalue_2))
          (UserInterface|Viewport|AddtoViewport _output_get_2 0)
          (Utilities|Array|Add (Variables|Default|GetAll%20WIdgets) _output_get_2))))
    (:then_2
      ;[0.15 0.03516 0.03516 0.5] Main Menu
      (bind _returnvalue_3 (UserInterface|CreateWidget "/Game/1_MyWorkingSpace/UI/V2/menuV2.menuV2_C"))
      (Utilities|IsValid _returnvalue_3
        (:Is%20Valid
          (bind _output_get_3 (Variables|Widgets|SetMM_MainMenu _returnvalue_3))
          (UserInterface|Viewport|AddtoViewport _output_get_3 0)
          (Utilities|Array|Add (Variables|Default|GetAll%20WIdgets) _output_get_3))))
    (:then_3
      (bind _returnvalue_4 (UserInterface|CreateWidget "/Game/1_MyWorkingSpace/UI/V2/map.map_C"))
      (bind _output_get_4 (Variables|Widgets|SetMM_StoryMap _returnvalue_4))
      (UserInterface|Viewport|AddtoViewport _output_get_4 0)
      (Utilities|Array|Add (Variables|Default|GetAll%20WIdgets) _output_get_4))
    (:then_4
      (bind _returnvalue_5 (UserInterface|CreateWidget "/Game/1_MyWorkingSpace/UI/V2/Shop.Shop_C"))
      (bind _output_get_5 (Variables|Widgets|SetMM_Shop _returnvalue_5))
      (UserInterface|Viewport|AddtoViewport _output_get_5 0)
      (Utilities|Array|Add (Variables|Default|GetAll%20WIdgets) _output_get_5))
    (:then_5
      (bind _returnvalue_6 (UserInterface|CreateWidget "/Game/1_MyWorkingSpace/UI/V2/16Settings_WB.16Settings_WB_C"))
      (bind _output_get_6 (Variables|Widgets|SetMM_Setting _returnvalue_6))
      (UserInterface|Viewport|AddtoViewport _output_get_6 0)
      (Utilities|Array|Add (Variables|Default|GetAll%20WIdgets) _output_get_6))
    (:then_7
      (bind _returnvalue_7 (UserInterface|CreateWidget "/Game/1_MyWorkingSpace/UI/V2/Gmail.Gmail_C"))
      (bind _output_get_7 (Variables|Widgets|SetMM_Gmail _returnvalue_7))
      (UserInterface|Viewport|AddtoViewport _output_get_7 0)
      (Utilities|Array|Add (Variables|Default|GetAll%20WIdgets) _output_get_7))
    (:then_8
      (bind _returnvalue_8 (UserInterface|CreateWidget "/Game/1_MyWorkingSpace/UI/V2/Harbore.Harbore_C"))
      (bind _output_get_8 (Variables|Widgets|SetMM_Harbore _returnvalue_8))
      (UserInterface|Viewport|AddtoViewport _output_get_8 0)
      (Utilities|Array|Add (Variables|Default|GetAll%20WIdgets) _output_get_8))
    (:then_9
      (bind _returnvalue_9 (UserInterface|CreateWidget "/Game/1_MyWorkingSpace/UI/V2/23Died_WB.23Died_WB_C"))
      (Utilities|IsValid _returnvalue_9
        (:Is%20Valid
          (bind _output_get_9 (Variables|Widgets|SetDeath%20UI _returnvalue_9))
          (UserInterface|Viewport|AddtoViewport _output_get_9 0)
          (Utilities|Array|Add (Variables|Default|GetAll%20WIdgets) _output_get_9))))
    (:then_10
      (bind _returnvalue_10 (UserInterface|CreateWidget "/Game/1_MyWorkingSpace/UI/V2/Victory.Victory_C"))
      (Utilities|IsValid _returnvalue_10
        (:Is%20Valid
          (bind _output_get_10 (Variables|Widgets|SetVectory%20UI _returnvalue_10))
          (UserInterface|Viewport|AddtoViewport _output_get_10 0)
          (Utilities|Array|Add (Variables|Default|GetAll%20WIdgets) _output_get_10))))
    (:then_11
      ;[0.15 0.15 0.15 0.5] Set all widgets to Collapse at start
      (for _array_element _all_widgets
        (Widget|SetVisibility _array_element "Collapsed"))
      (Variables|Default|SetAll%20WIdgets%20Temp _all_widgets)
      (CallFunction|ChangeUILayout (Variables|Default|GetUI%20Mode)))))

(fn ConstructionScript)

(fn GetPatrolPath
  (return 0))