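; Game mode for the turret test field level that sets up the player's UI and touch input when play begins.
; BeginPlay retries on short delays until the turret test field player controller and test HUD are valid, then switches the HUD layout and enables touch.
; GetPC and GetHUD are lazy getters that cast and cache their references.
; GetPatrolPath is an empty stub.
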(event EventTick
  (params (DeltaSeconds :type Float%20%28single-precision%29)))

(event EventBeginPlay
  (Utilities|FlowControl|Sequence
    (:then_0
      (bind _output_get (CallFunction|GetPC :!label _label))
      (Utilities|IsValid _output_get
        (:Is%20Valid
          (bind _output_get_2 (CallFunction|GetHUD :!label _label_2))
          (Utilities|IsValid _output_get_2
            (:Is%20Valid
              (Utilities|FlowControl|Delay 0.5)
              (Default|ChangeUILayout (Variables|Default|GetAs%20BP%20HUD%20Test) "NewEnumerator0")
              (Variables|/Game/1_MyWorkingSpace/BluePrint/GameFunctions/TestField/BP_WS_TurretTestField.BP_WS_TurretTestField_C|SetTouch%20Is%20Allowed? _output_get true))
            (:Is%20Not%20Valid
              (Utilities|FlowControl|Delay 0.2)
              (goto _label_2))))
        (:Is%20Not%20Valid
          (Utilities|FlowControl|Delay 0.2)
          (goto _label))))))

(fn ConstructionScript)

(fn GetHUD
  (Utilities|IsValid (Variables|Default|GetAs%20BP%20HUD%20Test)
    (:Is%20Valid
      _)
    (:Is%20Not%20Valid
      (bind _asbp_hud_test (Utilities|Casting|CastToBP_HUD_Test (HUD|GetHUD (Game|GetPlayerController 0)))
        (:then
          (Variables|Default|SetAs%20BP%20HUD%20Test _asbp_hud_test))
        (:CastFailed
          (return (Variables|Default|GetAs%20BP%20HUD%20Test))))))
  (return (Variables|Default|GetAs%20BP%20HUD%20Test)))

(fn GetPC
  (Utilities|IsValid (Variables|Default|GetAs%20BP%20WS%20Turret%20Test%20Field)
    (:Is%20Valid
      _)
    (:Is%20Not%20Valid
      (bind _asbp_ws_turret_test_field (Utilities|Casting|CastToBP_WS_TurretTestField (Game|GetPlayerController 0))
        (:then
          (bind _output_get (Variables|Default|SetAs%20BP%20WS%20Turret%20Test%20Field _asbp_ws_turret_test_field)))
        (:CastFailed
          (return (Variables|Default|GetAs%20BP%20WS%20Turret%20Test%20Field))))))
  (return _output_get))

(fn GetPatrolPath
  (return 0))