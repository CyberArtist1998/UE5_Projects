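; BP_CameraAnimation plays intro and outro camera animation sequences on the first player's camera through the Engine Cameras Subsystem.
; Each of its two custom events starts its sequence, waits slightly longer than the expected five-second length, then checks whether the animation is still active.
; It prints a debug status, with the outro reusing the intro's message text, then requests a non-immediate stop on that animation handle.
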(event Custom|Camera%20Animation%20-%20Outro
  (bind _returnvalue (Game|GetPlayerController 0))
  (bind _returnvalue_2 (Subsystems|GetEngineCamerasSubsystem))
  (bind _returnvalue_3 (Class|EngineCamerasSubsystem|PlayCameraAnimation _returnvalue_2 _returnvalue "/Game/1_MyWorkingSpace/BluePrint/GameFunctions/CA_Outro.CA_Outro"))
  (Utilities|FlowControl|Delay 5.1) ; Becase the whole sequnce is 5 seconds
  (if (Class|EngineCamerasSubsystem|IsCameraAnimationActive _returnvalue_2 _returnvalue _returnvalue_3)
    (Development|PrintString "Into Camera Animation stoped midway")
    (else
      (Development|PrintString "Into Camera Animation completed")))
  (Class|EngineCamerasSubsystem|StopCameraAnimation _returnvalue_2 _returnvalue _returnvalue_3 false))

(event Custom|Camera%20Animation%20-%20Intro
  (bind _returnvalue (Game|GetPlayerController 0))
  (bind _returnvalue_2 (Subsystems|GetEngineCamerasSubsystem))
  (bind _returnvalue_3 (Class|EngineCamerasSubsystem|PlayCameraAnimation _returnvalue_2 _returnvalue "/Game/1_MyWorkingSpace/BluePrint/GameFunctions/CA_Intro.CA_Intro"))
  (Utilities|FlowControl|Delay 5.1) ; Becase the whole sequnce is 5 seconds
  (if (Class|EngineCamerasSubsystem|IsCameraAnimationActive _returnvalue_2 _returnvalue _returnvalue_3)
    (Development|PrintString "Into Camera Animation stoped midway")
    (else
      (Development|PrintString "Into Camera Animation completed")))
  (Class|EngineCamerasSubsystem|StopCameraAnimation _returnvalue_2 _returnvalue _returnvalue_3 false))

(fn ConstructionScript)