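; BP_ScortShip is an AI-controlled escort ship that takes damage and plays a staged explosion on death.
; BeginPlay initializes its health component, and AnyDamage forwards damage to it.
; DeathExplosion, also triggered by the M key, runs once through a collapsed graph that spawns delayed Niagara blasts at random points around the mesh with 2D sounds, ending with a larger one.
; The AI controller then unpossesses the ship.
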(event Custom|DeathExplosion
  ;[1 0 0.0133] Death / Damage
  (Utilities|FlowControl|DoOnce false
    (:Completed
      (|CollapseGraph (Variables|Default|GetStaticMesh))
      (Pawn|UnPossess (AI|GetAIController self)))))

(event Game|Damage|EventAnyDamage
  (params (Damage :type Float%20%28single-precision%29) (DamageType :type Damage%20Type%20Object%20Reference) (InstigatedBy :type Controller%20Object%20Reference) (DamageCauser :type Actor%20Object%20Reference))
  ;[1 0 0.0133] Death / Damage
  (Default|RunTime-HealthUpdate (Variables|Default|GetWSHealthComp) Damage "NewEnumerator0"))

(event EventBeginPlay
  (Default|Initial-ActorMaxHealth (Variables|Default|GetWSHealthComp) "NewEnumerator4"))

(event Input|KeyboardEvents|M
  (params (Key :type Key%20Structure))
  ;[1 0 0.0133] Death / Damage
  (:Pressed
    (Utilities|FlowControl|DoOnce false
      (:Completed
        (|CollapseGraph (Variables|Default|GetStaticMesh))
        (Pawn|UnPossess (AI|GetAIController self))))))

(fn ConstructionScript
  (|CallParentFunction))