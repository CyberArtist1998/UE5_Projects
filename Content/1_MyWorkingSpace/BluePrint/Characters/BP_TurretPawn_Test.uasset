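; Test pawn for a camera-aimed 76mm turret that fires projectiles tagged to target enemies.
; On Tick, base yaw and barrel pitch interpolate toward the front camera, which holds its last rotation while the turret is offline.
; Z or custom events fire one shot, with a 0.2-second ShotCount reset, spawning projectile, Niagara effects, camera shake and sound.
; Health and patrol functions are empty; Turret Rotation_2 largely duplicates the rotation logic.
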(event Custom|FirePattern
  ;[1 0.46 0] Turret
  (if (Variables|FrontTurrent|GetCanFire?)
    (Variables|FrontTurrent|SetCanFire? true :!label _label)
    (if (<= (Variables|Default|GetShotCount) 0)
      (Math|Integer|IncrementInt (Variables|Default|GetShotCount)
        (:%20%20
          (CallFunction|Fire76mm)
          (goto _label)))
      (else
        (Utilities|FlowControl|Delay 0.2)
        (Variables|Default|SetShotCount 0)
        (Variables|FrontTurrent|SetCanFire? true)))))

(event Custom|Fire76mm
  (bind _turret_76mm_barrel (Variables|Default|GetTurret_76mm_Barrel))
  (bind _returnvalue (Transformation|GetWorldRotation _turret_76mm_barrel))
  ;[1 0.46 0] Turret
  (Variables|Default|SetMZForwardVector (Transformation|GetWorldLocation (Variables|Default|Get76mm_FN_SC)))
  (Game|SpawnActorfromClass "/Game/1_MyWorkingSpace/BluePrint/Weapons/BP_WS_ProjectileParent.BP_WS_ProjectileParent_C" (Math|Transform|MakeTransform (Variables|Default|GetMZForwardVector) _returnvalue (* (Variables|FrontTurrent|GetBulletScaleMultip) (Variables|FrontTurrent|GetBulletScale))) "Undefined" "MultiplyWithRoot" 0 1e+01 0.2 "Enemy" self)
  (Niagara|SpawnSystematLocation "/Game/1_MyWorkingSpace/VFX/MuzzleFlash/NS_MuzzleFlash_Tank_Mashingun_1.NS_MuzzleFlash_Tank_Mashingun_1" (Variables|Default|GetMZForwardVector) _returnvalue (* 5 "1.000000,1.000000,1.000000"))
  (Niagara|SpawnSystematLocation "/Game/1_MyWorkingSpace/VFX/Shells/NS_Shells_APC_1.NS_Shells_APC_1" (Transformation|GetWorldLocation (Variables|Default|Get76mm_FN_SC)) "0, 0, 0" (* 10 "1.000000,1.000000,1.000000"))
  (if true
    _
    (else
      (Rendering|Debug|DrawDebugSphere (Variables|Default|GetMZForwardVector) 1e+02 12 "(R=1.000000,G=1.000000,B=1.000000,A=1.000000)" 2.0)
      (Rendering|Debug|DrawDebugSphere (Variables|Default|GetMZForwardVector) 1e+02 12 "(R=1.000000,G=1.000000,B=1.000000,A=1.000000)" 2.0)))
  (Camera|PlayWorldCameraShake "/Game/1_MyWorkingSpace/BluePrint/GameFunctions/CameraManager/BP_CameraShake_Bullets.BP_CameraShake_Bullets_C" (Transformation|GetActorLocation) 0.0 5e+04 0.5)
  (Audio|PlaySoundatLocation "/Game/1_MyWorkingSpace/Sound/SoundCue/SC_TurretShooting.SC_TurretShooting" (Transformation|GetWorldLocation (Variables|Default|Get76mm_FN_MF)) "0, 0, 0" 1.0 1.0 0.0 0 0 0 0))

(event Custom|UpdateTurretRotation
  (bind _frontturretcam (Variables|Default|GetFrontTurretCam))
  (bind _turret_76mm_barrel (Variables|Default|GetTurret_76mm_Barrel))
  (bind _returnvalue (Transformation|GetWorldRotation _frontturretcam))
  ;[1 0.46 0] Turret
  (if (Variables|Default|GetTurret%20Online?) ; True: Camera is Active and Player is controling it\nFalse : Camera and Turret is offline and they should stay in their last position
    ;;[0.15 0.15 0.742 0.5] Camera states
    (Variables|Default|SetCamera%20-Value%20X%20%28Roll%29 (.roll _returnvalue))
    (bind _output_get (Variables|Default|SetCamera%20-%20Value%20Y%20%28Pitch%29 (.pitch _returnvalue)))
    (bind _output_get_2 (Variables|Default|SetCamera%20-Value%20Z%20%28Yaw%29 (.yaw _returnvalue)))
    (Utilities|FlowControl|Sequence
      (:then_0
        ;;[0.15 0.15 0.742 0.5] Turret Base Rotation - Recive 'Z' of camera
        (Variables|Default|SetTurret%20-%20Value%20Z (Math|Interpolation|FInterpTo (.yaw (Transformation|GetWorldRotation (Variables|Default|GetTurret_76mm_Base))) _output_get_2 (Utilities|Time|GetWorldDeltaSeconds) (Variables|Default|GetInterp%20Speed)))
        (Transformation|SetWorldRotation (Variables|Default|GetTurret_76mm_Base) (Math|Rotator|MakeRotator 0.0 0.0 (Variables|Default|GetTurret%20-%20Value%20Z)) false false))
      (:then_1
        (bind _output_get_3 (Variables|Default|SetTurret%20-%20Value%20Y (.pitch (Math|Interpolation|RInterpTo (Math|Rotator|MakeRotator 0.0 (.pitch (Transformation|GetWorldRotation _turret_76mm_barrel)) 0.0) (Math|Rotator|MakeRotator 0.0 _output_get 0.0) (Utilities|Time|GetWorldDeltaSeconds) (Variables|Default|GetInterp%20Speed)))))
        (Transformation|SetWorldRotation _turret_76mm_barrel (Math|Rotator|MakeRotator 0.0 _output_get_3 (Variables|Default|GetTurret%20-%20Value%20Z)) false false)))
    (else
      (Transformation|SetWorldRotation (Variables|Default|GetFrontTurretCam) (Math|Rotator|MakeRotator (Variables|Default|GetCamera%20-Value%20X%20%28Roll%29) (Variables|Default|GetCamera%20-%20Value%20Y%20%28Pitch%29) (Variables|Default|GetCamera%20-Value%20Z%20%28Yaw%29)) false false))))

(event Custom|CustomEvent
  ;[1 0.46 0] Turret
  (if (Variables|FrontTurrent|GetCanFire?)
    (Variables|FrontTurrent|SetCanFire? true :!label _label)
    (if (<= (Variables|Default|GetShotCount) 0)
      (Math|Integer|IncrementInt (Variables|Default|GetShotCount)
        (:%20%20
          (CallFunction|Fire76mm)
          (goto _label)))
      (else
        (Utilities|FlowControl|Delay 0.2)
        (Variables|Default|SetShotCount 0)
        (Variables|FrontTurrent|SetCanFire? true)))))

(event EventBeginPlay)

(event EventTick
  (params (DeltaSeconds :type Float%20%28single-precision%29))
  (CallFunction|UpdateTurretRotation))

(event Input|KeyboardEvents|Z
  (params (Key :type Key%20Structure))
  ;[1 0.46 0] Turret
  (:Pressed
    (if (Variables|FrontTurrent|GetCanFire?)
      (Variables|FrontTurrent|SetCanFire? true :!label _label)
      (if (<= (Variables|Default|GetShotCount) 0)
        (Math|Integer|IncrementInt (Variables|Default|GetShotCount)
          (:%20%20
            (CallFunction|Fire76mm)
            (goto _label)))
        (else
          (Utilities|FlowControl|Delay 0.2)
          (Variables|Default|SetShotCount 0)
          (Variables|FrontTurrent|SetCanFire? true))))))

(fn ConstructionScript)

(fn BPIWFHealth
  (params (BPI_WF%20Heaalth%20value%20input :type Integer))
  (return))

(fn GetPatrolPath
  (return 0))