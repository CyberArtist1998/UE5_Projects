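; Enemy DDG5 turret that aims at the player warship and fires projectiles while the master AI reports it in range.
; BeginPlay retries finding the player every two seconds and binds to the BP_MasterAISkInRot range event.
; A Delay on Tick paces aim and fire, rotating Body and Barrel from the look-at pitch alone.
; Each shot spawns a Player-tagged projectile along the full look-at rotation, with muzzle flash, sound and debug sphere.
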(event Custom|CustomEvent
  (params (Is%20Enemy%20In%20Range? :type Boolean))
  (bind _output_get (Variables|Default|SetIs%20Enemy%20In%20Range? Is%20Enemy%20In%20Range?))
  (if _output_get
    (Variables|Default|SetCanFire? true)
    (else
      (Variables|Default|SetCanFire? false))))

(event Custom|SpawnPojectile
  ;[1 1 1] Comment
  (bind _output_get (Variables|Default|SetMuzzelLocation (Transformation|GetWorldLocation (Variables|Default|Get76mm_FN_SC))))
  (if false
    (Development|PrintString (Utilities|String|ToString(Vector) _output_get)))
  (Game|SpawnActorfromClass "/Game/1_MyWorkingSpace/BluePrint/Weapons/BP_WS_ProjectileParent.BP_WS_ProjectileParent_C" (Math|Transform|MakeTransform (Variables|Default|GetMuzzelLocation) (Variables|Default|GetTurretLookingAtPlayer) "10.000000,10.000000,10.000000") "AlwaysSpawn" "MultiplyWithRoot" 0 1.0 0.2 "Player" self) ; BP_WS_ProjectileParent_Enemys
  (Niagara|SpawnSystematLocation "/Game/1_MyWorkingSpace/VFX/MuzzleFlash/NS_MuzzleFlash_Tank_Mashingun_1.NS_MuzzleFlash_Tank_Mashingun_1" (Variables|Default|GetMuzzelLocation) (Transformation|GetWorldRotation (Variables|Default|GetBarrel)))
  (if false
    _
    (else
      (Rendering|Debug|DrawDebugSphere (Variables|Default|GetMuzzelLocation) 1e+02 12 "(R=1.000000,G=1.000000,B=1.000000,A=1.000000)" 2.0)))
  (Audio|PlaySoundatLocation "/Game/1_MyWorkingSpace/Sound/شلیک_توپ.شلیک_توپ" (Transformation|GetWorldLocation (Variables|Default|Get76mm_FN_MF)) "0, 0, 0" 1.0 1.0 0.0 0 0 0 0))

(event Custom|FirePattern
  ;[1 1 1] Comment
  (if (Variables|Default|GetCanFire?)
    (CallFunction|SpawnPojectile)))

(event EventBeginPlay
  (Utilities|FlowControl|Sequence
    (:then_0
      (CallFunction|GetMasterAI)
      (bind _as_bp_warship_main_player (CallFunction|GetPlayerWarship :!label _label))
      (Utilities|IsValid _as_bp_warship_main_player
        (:Is%20Valid
          (Variables|Default|SetTarget%20Acuired? true))
        (:Is%20Not%20Valid
          (Variables|Default|SetTarget%20Acuired? false)
          (Utilities|FlowControl|Delay 2.0)
          (goto _label))))
    (:then_1
      (EventDispatchers|BindEventtoEDIsEnemyinRange? (Variables|Getter|GetBP%20Master%20AI) (delegate Custom|CustomEvent)))))

(event EventTick
  (params (DeltaSeconds :type Float%20%28single-precision%29))
  (if (and (Variables|Default|GetTarget%20Acuired?) (Variables|Default|GetIs%20Enemy%20In%20Range?))
    (Utilities|FlowControl|Delay 0.5)
    (bind _output_get (Variables|Default|SetTurretLookingAtPlayer (Math|Rotator|FindLookatRotation (Transformation|GetWorldLocation (Variables|Default|GetBody)) (Transformation|GetActorLocation (Variables|Default|GetAs%20BP%20Warship%20Main%20Player)))))
    (Transformation|SetWorldRotation (Variables|Default|GetBody) (Math|Rotator|MakeRotator 0.0 0.0 (.pitch _output_get)) false false)
    (Transformation|SetWorldRotation (Variables|Default|GetBarrel) (Math|Rotator|MakeRotator (* (.pitch _output_get) -1.0) 0.0 0.0) false false)
    ;[1 0.7876 0.5244] Update Rotation - Fire Order
    (CallFunction|FirePattern)))

(fn ConstructionScript)

(fn GetMasterAI
  (Utilities|IsValid 0
    (:Is%20Valid
      _)
    (:Is%20Not%20Valid
      (bind _returnvalue (Actor|GetActorOfClass "/Game/1_MyWorkingSpace/BluePrint/Characters/BP_MasterAI-SkInRot.BP_MasterAI-SkInRot_C"))
      (bind _output_get (Variables|Getter|SetBP%20Master%20AI _returnvalue))))
  (return _output_get))

(fn GetPlayerWarship
  (Utilities|IsValid (Variables|Default|GetAs%20BP%20Warship%20Main%20Player)
    (:Is%20Valid
      _)
    (:Is%20Not%20Valid
      (bind _asbp_warship_main_player (Utilities|Casting|CastToBP_WarshipMainPlayer (Game|Player|GetPlayerPawn 0))
        (:then
          (bind _output_get (Variables|Default|SetAs%20BP%20Warship%20Main%20Player _asbp_warship_main_player)))
        (:CastFailed
          (return (Variables|Default|GetAs%20BP%20Warship%20Main%20Player))))))
  (return _output_get))