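; Parent Blueprint for air missiles that home on a target component and damage actors carrying a target tag.
; On BeginPlay it reads its DT_Damage row by actor category, assigns the homing target, then sets a very high homing acceleration after a short delay.
; Box overlap with a tagged actor applies the table damage, spawns explosion effect and sound, and destroys the missile.
; The construction script caches the warship player controller.
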(event OnComponentBeginOverlap(Box)
  (params (OverlappedComponent :type Primitive%20Component%20Object%20Reference) (OtherActor :type Actor%20Object%20Reference) (OtherComp :type Primitive%20Component%20Object%20Reference) (OtherBodyIndex :type Integer) (bFromSweep :type Boolean) (SweepResult :type Hit%20Result%20Structure%20%28by%20ref%29))
  (bind _returnvalue (Transformation|GetActorLocation))
  (Utilities|IsValid OtherActor
    (:Is%20Valid
      ;[1 0 0.005087] Comment
      (if (Actor|ActorHasTag OtherActor (Variables|Default|GetTargetTag))
        (Game|Damage|ApplyDamage OtherActor (Utilities|Struct|BreakS_Damage (stale EventBeginPlay _returnvalue)) 0 0 "/Script/Engine.DamageType")
        (Niagara|SpawnSystematLocation "/Game/1_MyWorkingSpace/VFX/Destroyed/NS_Expl_Tank_1.NS_Expl_Tank_1" _returnvalue "0, 0, 0" (* "1.000000,1.000000,1.000000" 5))
        (Audio|SpawnSoundatLocation "/Game/1_MyWorkingSpace/Sound/SoundCue/SC_RockHit.SC_RockHit" _returnvalue "0, 0, 0" 1.0 1.0 0.0 0 0)
        (Actor|DestroyActor)))))

(event EventBeginPlay
  (bind _returnvalue (Utilities|GetDataTableRow "/Game/1_MyWorkingSpace/Data/DT_Damage.DT_Damage" (Variables|Default|GetActor%20Category))
    (:then
      (if false ; Debugger
        (Rendering|Debug|DrawDebugSphere (Transformation|GetActorLocation) 8e+02 15 "(R=0.000000,G=1.000000,B=0.210027,A=1.000000)" 1.0 25.0)
        (Rendering|Debug|DrawDebugSphere (Variables|Default|GetTarget%20World%20Location) 1.8e+03 15 "(R=1.000000,G=0.000000,B=0.053521,A=1.000000)" 1.0 25.0))
      (Variables|/Script/Engine.ProjectileMovementComponent|SetHomingTargetComponent (Variables|MyProjectile|GetProjectileMovement) (Variables|Default|GetTarget%20Scene%20Component))
      (Utilities|FlowControl|Delay 2.0)
      (Variables|/Script/Engine.ProjectileMovementComponent|SetHomingAccelerationMagnitude (Variables|MyProjectile|GetProjectileMovement) 1e+05))))

(fn ConstructionScript
  (CallFunction|CasttoControler))

(fn CasttoControler
  (Utilities|IsValid (Variables|Default|GetAs%20BP%20WS%20Player%20Controler)
    (:Is%20Valid
      _)
    (:Is%20Not%20Valid
      (bind _asbp_ws_player_controler (Utilities|Casting|CastToBP_WarshipPlayerControler (Game|GetPlayerController 0))
        (:then
          (bind _output_get (Variables|Default|SetAs%20BP%20WS%20Player%20Controler _asbp_ws_player_controler)))
        (:CastFailed
          (return 0)))))
  (return _output_get))