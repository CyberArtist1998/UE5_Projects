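; Warship missile launcher Blueprint that fires missiles at the nearest opposing target, for player or enemy owners.
; BPIWFFireMissiles sets team tags from ownership, then EnemyDetector finds the closest tagged ship and checks DetectionRange, drawing a debug sphere.
; In range, a delayed loop calls MissileFire twice before cooling down.
; MissileFire's FlipFlop wires only output A, so alternate calls spawn a target-aware missile with VFX, sound and camera shake.
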(event Custom|EnemyDetector
  ;[1 1 1] Comment
  ;;[1 1 1] Comment
  (switch Utilities|FlowControl|Switch|SwitchonE_Tag (Variables|Default|GetSelect%20Tag)
    (:NewEnumerator0
      (bind _outactors (Actor|GetAllActorsOfClasswithTag "/Game/1_MyWorkingSpace/BluePrint/Characters/BP_WarshipMainPlayer.BP_WarshipMainPlayer_C" "Player"))
      (Variables|Default|SetOut%20Actors_1 _outactors))
    (:NewEnumerator1
      (bind _outactors_2 (Actor|GetAllActorsOfClasswithTag "/Game/1_MyWorkingSpace/BluePrint/Characters/BP_MasterAI-SkInRot.BP_MasterAI-SkInRot_C" "Enemy"))
      (Variables|Default|SetOut%20Actors_1 _outactors_2)))
  (|Debug-DetectionRangeSphare)
  (if (not (== (Utilities|Array|Length (Variables|Default|GetOut%20Actors_1)) 0))
    (Utilities|FlowControl|Sequence
      (:then_0
        (Variables|Default|SetClosest%20Target%20In%20Renge (.ReturnValue (Actor|FindNearestActor (Transformation|GetWorldLocation (Variables|Default|GetSKM_MissileLauncher_MK4)) (Variables|Default|GetOut%20Actors_1))))
        (if (<= (.Distance (Actor|FindNearestActor (Transformation|GetWorldLocation (Variables|Default|GetSKM_MissileLauncher_MK4)) (Variables|Default|GetOut%20Actors_1))) (Variables|Default|GetDetection%20Range))
          (Variables|Default|SetTarget%20in%20range%20of%20missile? true)
          (Variables|Default|SetTarget%20World%20Location (Transformation|GetActorLocation (Variables|Default|GetClosest%20Target%20In%20Renge)))
          (else
            (Variables|Default|SetTarget%20in%20range%20of%20missile? false :!label _label)))))
    (else
      (goto _label))))

(event Custom|MissileFire
  (params (Spawner%20Tag :type Name) (Target%20Tag :type Name))
  (bind _76mm_fn_mf (Variables|Default|Get76mm_FN_MF))
  (bind _returnvalue (Transformation|GetWorldTransform _76mm_fn_mf))
  (Utilities|FlowControl|FlipFlop
    (:A
      (Variables|Default|SetMissileFirelocation (Variables|Default|Get76mm_FN_SC))
      (Niagara|SpawnSystematLocation "/Game/1_MyWorkingSpace/VFX/Projectiles/NS_Rocket_Start.NS_Rocket_Start" (.location _returnvalue) (.rotation _returnvalue) (* "1.000000,1.000000,1.000000" 2))
      (Game|SpawnActorfromClass "/Game/1_MyWorkingSpace/BluePrint/Weapons/BP_AirMissileParent.BP_AirMissileParent_C" (Math|Transform|MakeTransform (.location (Transformation|GetWorldTransform (Variables|Default|GetMissileFirelocation))) (.rotation (Transformation|GetWorldTransform (Variables|Default|GetMissileFirelocation))) (* "1.000000,1.000000,1.000000" 2)) "Undefined" "MultiplyWithRoot" 0 5.0 Spawner%20Tag Target%20Tag (Variables|Default|GetTarget%20World%20Location) (Actor|GetComponentbyClass (Variables|Default|GetClosest%20Target%20In%20Renge) "/Script/Engine.SceneComponent") "Enemy_Missile" self)
      (Camera|PlayWorldCameraShake "/Game/1_MyWorkingSpace/BluePrint/GameFunctions/CameraManager/BP_CameraShake_Missiles.BP_CameraShake_Missiles_C" (.location (Transformation|GetWorldTransform (Variables|Default|GetMissileFirelocation))) 0.0 5e+04 0.5)
      (Audio|PlaySoundatLocation "/Game/1_MyWorkingSpace/Sound/SoundCue/SC_RockLauncher.SC_RockLauncher" (.location (Transformation|GetWorldTransform (Variables|Default|GetMissileFirelocation))) "0, 0, 0" 1.0 1.0 0.0 0 0 0 0))))

(event EventBPIWFFireMissiles
  (params (Owner%20is%20Player? :type Boolean) (Owner%20Ref :type Actor%20Object%20Reference))
  ;[1 1 1] به جای این همه کد میشه یک ایسنتیگیتور گذاشت!!!
  ;[1 0 0.005087] Owner Is Player? (True) > Select (0) > Option (0) Player
  ; Owner Is Player? (False) > Select (1) > Option (1) Enemy
  (bind _output_get (Variables|Default|SetSelect%20Tag (select Owner%20is%20Player? "NewEnumerator1" "NewEnumerator0")))
  (switch Utilities|FlowControl|Switch|SwitchonE_Tag _output_get
    (:NewEnumerator0
      (Variables|Default|SetSpawner%20Tag "Enemy")
      (Variables|Default|SetTarget%20Tag "Player"))
    (:NewEnumerator1
      (Variables|Default|SetSpawner%20Tag "Player")
      (Variables|Default|SetTarget%20Tag "Enemy")))
  (CallFunction|EnemyDetector)
  (if (Variables|Default|GetTarget%20in%20range%20of%20missile?)
    (if (Variables|Default|GetCanFireMissile?)
      (Variables|Default|SetCanFireMissile? false :!label _label)
      ;[0 0.7891 1] 3 Shots
      (if (<= (Variables|Default|GetMissileCount) 1)
        (Math|Integer|IncrementInt (Variables|Default|GetMissileCount)
          (:%20%20
            (CallFunction|MissileFire (Variables|Default|GetSpawner%20Tag) (Variables|Default|GetTarget%20Tag))
            (Utilities|FlowControl|Delay 0.8)
            (goto _label)))
        (else
          (Utilities|FlowControl|Delay 5.0)
          (Variables|Default|SetMissileCount 0)
          (Variables|Default|SetCanFireMissile? true))))
    (else
      (Development|PrintString "There is no target"))))

(fn ConstructionScript)

(fn CameraData)

(fn CasttoControler
  (Utilities|IsValid (Variables|Default|GetAs%20BP%20WS%20Player%20Controler)
    (:Is%20Valid
      _)
    (:Is%20Not%20Valid
      (bind _asbp_ws_player_controler (Utilities|Casting|CastToBP_WarshipPlayerControler (Game|GetPlayerController 0))
        (:then
          (bind _output_get (Variables|Default|SetAs%20BP%20WS%20Player%20Controler _asbp_ws_player_controler)))
        (:CastFailed
          (return 0)))))
  (return _output_get))

(fn GetPatrolPath
  (return 0))