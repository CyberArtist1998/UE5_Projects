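; Parent projectile Blueprint for weapons that damages tagged targets on contact.
; It attaches a Niagara trail at BeginPlay; on box overlap, it caches hit data and rolls a critical.
; Actors carrying TargetTag receive plain damage and a Niagara explosion, then the projectile destroys itself.
; Surface-based effects, decals, sounds and critical-aware point damage exist only as disconnected or uncalled logic.
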(event OnComponentBeginOverlap(Box)
  (params (OverlappedComponent :type Primitive%20Component%20Object%20Reference) (OtherActor :type Actor%20Object%20Reference) (OtherComp :type Primitive%20Component%20Object%20Reference) (OtherBodyIndex :type Integer) (bFromSweep :type Boolean) (SweepResult :type Hit%20Result%20Structure%20%28by%20ref%29))
  (bind _other (Variables|Default|GetOther))
  (|Getter OtherActor OtherComp SweepResult)
  (Utilities|FlowControl|Sequence
    (:then_0
      (Utilities|IsValid _other
        (:Is%20Valid
          ;[0 0.3977 0.4323 0.5] Debugger
          (if false ; Debug
            (Development|PrintString (Utilities|GetDisplayName _other)))
          (if (Actor|ActorHasTag (Variables|Default|GetOther) (Variables|Default|GetTarget%20Tag))
            (Game|Damage|ApplyDamage (Variables|Default|GetOther) (* 1.0 (Variables|Attributes|GetDamage)) 0 0 "/Script/Engine.DamageType")
            ;[0.15 0.15 0.15 0.5] Spawn Niagara
            (Niagara|SpawnSystematLocation "/Game/1_MyWorkingSpace/VFX/Destroyed/NS_Expl_Tank_1.NS_Expl_Tank_1" (.Location (Collision|BreakHitResult (Variables|Default|GetHit))) "0, 0, 0" (* (Variables|Default|GetScale%20of%20HitLocation) 1))
            (Actor|DestroyActor)))))))

(event EventBeginPlay
  (Niagara|SpawnSystemAttached "/Game/1_MyWorkingSpace/VFX/Trace/NS_Trace.NS_Trace" (Variables|Default|GetMesh) "None" "0, 0, 0" "0, 0, 0" "KeepRelativeOffset" false))

(fn ConstructionScript)

(fn PhysicMatDetermination)

(fn DecalSetFadeScreenSize
  (params (Decal :type Decal%20Component%20Object%20Reference))
  (Utilities|IsValid Decal
    (:Is%20Valid
      (Rendering|Components|Decal|SetFadeScreenSize Decal 0.005) ; Prevent fading decals
    )))

(fn SpawnParticle
  (bind _hit (Variables|Default|GetHit))
  (bind (_bblockinghit _binitialoverlap _time _distance _location _impactpoint _normal _impactnormal _physmat _hitactor _hitcomponent _hitbonename) (Collision|BreakHitResult _hit))
  (Variables|Default|SetHit%20Component (.HitComponent (Collision|BreakHitResult (Variables|Default|GetHit))))
  (LocalVariables|SetHitRot (Math|Rotator|MakeRotfromZ (.ImpactNormal (Collision|BreakHitResult (Variables|Default|GetHit)))))
  (LocalVariables|SetParticle 0)
  (LocalVariables|SetScale "0, 0, 0")
  (Effects|SpawnEmitterAttached (LocalVariables|GetParticle) (Variables|Default|GetHit%20Component) _hitbonename _impactpoint (LocalVariables|GetHitRot) (LocalVariables|GetScale) "KeepWorldPosition" true "AutoRelease"))

(fn IsCriticalHit
  (return (>= (Math|Float|Truncate (Math|Float|MapRangeClamped (Variables|Attributes|GetCriticalHitRate) 0.0 1.0 0.0 1e+02)) (Math|Random|RandomIntegerinRange 0 100))))

(event Custom|AddImpulseToOther)