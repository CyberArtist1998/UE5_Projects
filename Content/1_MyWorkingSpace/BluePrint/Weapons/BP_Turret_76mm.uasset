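; 76mm turret weapon Blueprint that follows the player camera and fires projectiles.
; Each tick, while TurretOnline, base yaw and barrel pitch interpolate toward Camera1's world rotation; offline, the camera holds its last stored rotation.
; The shooting interface event and FirePattern share a ShotCount gate allowing one shot per short delay, despite a "3 Shots" note.
; Fire76mm spawns the projectile, muzzle flash and camera shake; debug spheres and prints remain active.
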(event Custom|FirePattern
  (if (Variables|Default|GetCanFire?)
    (Development|PrintString "Branch > True > Shooting" true true "(R=0.310000,G=0.000000,B=0.000000,A=1.000000)" 0.5)
    (Variables|Default|SetCanFire? true :!label _label)
    ;[0 0.7891 1] 3 Shots
    (if (<= (Variables|Default|GetShotCount) 0)
      (Math|Integer|IncrementInt (Variables|Default|GetShotCount)
        (:%20%20
          (CallFunction|Fire76mm)
          (goto _label)))
      (else
        (Utilities|FlowControl|Delay 0.6)
        (Variables|Default|SetShotCount 0)
        (Development|PrintString "Cooldown is finished" true true "(R=0.025149,G=0.310000,B=0.000000,A=1.000000)" 0.5)
        (Variables|Default|SetCanFire? true)))
    (else
      (Development|PrintString "In Cooldown" true true "(R=1.000000,G=0.000000,B=0.000000,A=1.000000)"))))

(event Custom|Fire76mm
  (bind _turret_76mm_base (Variables|Default|GetTurret_76mm_Base))
  (bind _returnvalue (Transformation|GetWorldRotation _turret_76mm_base))
  (Variables|Default|SetMZForwardVector (Transformation|GetWorldLocation (Variables|Default|Get76mm_FN_SC)))
  (Game|SpawnActorfromClass "/Game/1_MyWorkingSpace/BluePrint/Weapons/BP_WS_ProjectileParent.BP_WS_ProjectileParent_C" (Math|Transform|MakeTransform (Variables|Default|GetMZForwardVector) _returnvalue (* (Variables|Default|GetBulletScaleMultip) (Variables|Default|GetBulletScale))) "Undefined" "MultiplyWithRoot" 0 1e+01 0.2 "None" self)
  (Niagara|SpawnSystematLocation "/Game/1_MyWorkingSpace/VFX/MuzzleFlash/NS_MuzzleFlash_Tank_Mashingun_1.NS_MuzzleFlash_Tank_Mashingun_1" (Variables|Default|GetMZForwardVector) _returnvalue)
  (if false
    _
    (else
      (Rendering|Debug|DrawDebugSphere (Variables|Default|GetMZForwardVector) 1e+02 12 "(R=1.000000,G=1.000000,B=1.000000,A=1.000000)" 2.0)
      (Rendering|Debug|DrawDebugSphere (Variables|Default|GetMZForwardVector) 1e+02 12 "(R=1.000000,G=1.000000,B=1.000000,A=1.000000)" 2.0)))
  (Camera|PlayWorldCameraShake "/Game/1_MyWorkingSpace/BluePrint/GameFunctions/CameraManager/BP_CameraShake_Bullets.BP_CameraShake_Bullets_C" (Transformation|GetActorLocation) 0.0 5e+04 0.5)
  (Audio|PlaySoundatLocation "/Game/1_MyWorkingSpace/Sound/شلیک_توپ.شلیک_توپ" (Transformation|GetWorldLocation (Variables|Default|Get76mm_FN_MF)) "0, 0, 0" 1.0 1.0 0.0 0 0 0 0))

(event EventTick
  (params (DeltaSeconds :type Float%20%28single-precision%29))
  (Utilities|FlowControl|Sequence
    (:then_0
      (|TurretRotation))
    (:then_1
      (Utilities|FlowControl|Delay 0.5)
      (CallFunction|Fire76mm))))

(event EventBeginPlay)

(event EventBPIWFShootingBullets
  (if (Variables|Default|GetCanFire?)
    (Development|PrintString "Branch > True > Shooting" true true "(R=0.310000,G=0.000000,B=0.000000,A=1.000000)" 0.5)
    (Variables|Default|SetCanFire? true :!label _label)
    ;[0 0.7891 1] 3 Shots
    (if (<= (Variables|Default|GetShotCount) 0)
      (Math|Integer|IncrementInt (Variables|Default|GetShotCount)
        (:%20%20
          (CallFunction|Fire76mm)
          (goto _label)))
      (else
        (Utilities|FlowControl|Delay 0.6)
        (Variables|Default|SetShotCount 0)
        (Development|PrintString "Cooldown is finished" true true "(R=0.025149,G=0.310000,B=0.000000,A=1.000000)" 0.5)
        (Variables|Default|SetCanFire? true)))
    (else
      (Development|PrintString "In Cooldown" true true "(R=1.000000,G=0.000000,B=0.000000,A=1.000000)"))))

(fn ConstructionScript)

(fn CameraData)

(fn GetPatrolPath
  (return 0))