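; WSHpWidgetComp is a widget component that displays a health bar for its owning actor.
; On BeginPlay it finds the owner's WSHealthComp and passes it into a new WB_3DHpBar, which it sets as its widget, because the bar cannot find that component itself.
; Despite comments about enemy type, the bar class is fixed, and the PreventShowIfHpFull and HideHpBar nodes are unconnected.
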(event EventBeginPlay
  ;[0.5193 0 0.01923] WIdget Component gets the owner HealthComponent and create a  HealthBarWidget base on the passed enemy type. Becuase HealthBarWidget can not directly find and access owner healthComponent, it is nessecry.
  (bind _output_get (Variables|Default|SetOwner%20Component (Actor|GetComponentbyClass (Components|GetOwner) "/Game/1_MyWorkingSpace/BluePrint/Components/WSHealthComp.WSHealthComp_C")))
  (CallFunction|CreateWidgetforEnemy _output_get))

(fn CreateWidgetforEnemy
  (params (WSHealthComp :type WS%20Health%20Comp%20Object%20Reference))
  (bind _returnvalue (UserInterface|CreateWidget "/Game/1_MyWorkingSpace/UI/WB_3DHpBar.WB_3DHpBar_C" 0 0 WSHealthComp))
  (bind _output_get (Variables|Default|SetHpBarWidget-Big _returnvalue))
  (UserInterface|SetWidget _output_get)
  (Utilities|IsValid _output_get))