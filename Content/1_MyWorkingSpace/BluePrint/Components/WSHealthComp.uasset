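; Health component for warships, boats and escort ships that tracks health and alive state, with a hook to trigger GameMode game over.
; BeginPlay gets the owner and initializes max health by actor-type enum.
; Health updates apply clamped damage or medkit changes and broadcast a health-changed dispatcher.
; It is unfinished: the alive check tests the incoming amount, percent conversion returns zero, and data-table lookup and armor logic are largely unwired.
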(event EventBeginPlay
  (Utilities|FlowControl|Sequence
    (:then_0
      (bind _output_get (Variables|Default|SetOwnerActor (Components|GetOwner) :!label _label)) ; Get Owner Actor
      (Utilities|IsValid _output_get
        (:Is%20Valid
          (bind _returnvalue (Actor|GetActorOfClass (Utilities|GetClass _output_get)))
          (if (== _output_get _returnvalue)
            (CallFunction|Initial-ActorMaxHealth (Variables|Default|GetEnum_ActorName))))
        (:Is%20Not%20Valid
          (Utilities|FlowControl|Delay 0.2)
          (Variables|Default|SetisAlive true)
          (goto _label))))))

(fn Initial-StoreAllActorClassinArray
  (params (Owner :type Actor%20Object%20Reference))
  (bind _all_actors_class (Variables|Default|GetAll%20Actors%20Class))
  (Utilities|FlowControl|Sequence
    (:then_0
      (bind _returnvalue (Actor|GetActorOfClass "/Game/1_MyWorkingSpace/BluePrint/Characters/BP_MasterAI-SkInRot.BP_MasterAI-SkInRot_C"))
      (Variables|Default|SetTemp1 _returnvalue)
      (bind _returnvalue_2 (Actor|GetActorOfClass "/Game/1_MyWorkingSpace/BluePrint/Characters/BP_MasterAI-SmallBouts.BP_MasterAI-SmallBouts_C"))
      (Variables|Default|SetTemp2 _returnvalue_2)
      (bind _returnvalue_3 (Actor|GetActorOfClass "/Game/1_MyWorkingSpace/BluePrint/Characters/BP_ScortShip.BP_ScortShip_C"))
      (Variables|Default|SetTemp3 _returnvalue_3))
    (:then_1
      (Utilities|Array|Add _all_actors_class (Utilities|GetClass (Variables|Default|GetTemp1)))
      (Utilities|Array|Add _all_actors_class (Utilities|GetClass (Variables|Default|GetTemp2)))
      (Utilities|Array|Add _all_actors_class (Utilities|GetClass (Variables|Default|GetTemp3))))
    (:then_2
      (bind _returnvalue_4 (Class|DataTableFunctionLibrary|GetDataTableColumnasString "/Game/1_MyWorkingSpace/Data/DT_ActorsPropertis.DT_ActorsPropertis" "Class"))
      (LocalVariables|SetNewLocalVar _returnvalue_4))
    (:then_3
      (bind (_array_element _array_index) (Utilities|Array|ForEachLoopwithBreak (Variables|Default|GetAll%20Actors%20Class))
        (:LoopBody
          (if (== _array_element (Utilities|GetClass Owner))
            (bind _output_get (LocalVariables|SetNewLocalVar_0 _array_index)) ; 0 - MasterAi - EnemyWarship\n1- MasterAi  - SmallBoat\n2- ScortShip
          ))))))

(fn Initial-ActorMaxHealth
  (params (Selection :type E_ActorsName%20Enum :default "NewEnumerator3"))
  (bind _returnvalue (Utilities|Select :Index Selection :NewEnumerator3 "" :NewEnumerator0 "" :NewEnumerator1 "" :NewEnumerator4 ""))
  (bind _maxhealth (Utilities|Struct|BreakS_ActorsPropertis _returnvalue))
  (bind _output_get (Variables|Default|SetEnum_ActorName Selection))
  (switch Utilities|FlowControl|Switch|SwitchonE_ActorsName _output_get ; For start, MaxHealth and Health ar the same level
    (:NewEnumerator3
      (bind _output_get_2 (Variables|Default|SetMaxHealth _maxhealth :!label _label))
      (bind _output_get_3 (Variables|Default|SetHealth _output_get_2))
      (Variables|Default|SetHealthPercent (/ _output_get_3 _output_get_2)))
    (:NewEnumerator0
      (goto _label))
    (:NewEnumerator1
      (bind _output_get_4 (Variables|Default|SetMaxHealth _maxhealth))
      (bind _output_get_5 (Variables|Default|SetHealth _output_get_4))
      (Variables|Default|SetHealthPercent (/ _output_get_5 _output_get_4)))
    (:NewEnumerator4
      (goto _label))))

(fn RunTime-HealthUpdate
  (params (Damage%20Amount :type Float%20%28double-precision%29) (Damage%20Or%20Medickit :type E_HealthChange%20Enum :default "NewEnumerator0"))
  (bind _medkit_or_damage (Variables|Default|GetMedkit%20or%20Damage))
  (bind _isalive_ (CallFunction|RunTime-IsActorAlive? Damage%20Amount))
  (if _isalive_
    (switch Utilities|FlowControl|Switch|SwitchonE_HealthChange Damage%20Or%20Medickit
      (:NewEnumerator0
        (bind _currenthealthpercent (CallFunction|RunTime-HealthCalculation Damage%20Amount _medkit_or_damage))
        (Default|CallWSonHealthChanged _currenthealthpercent true))
      (:NewEnumerator1
        (CallFunction|RunTime-HealthCalculation Damage%20Amount _medkit_or_damage :!label _label)
        (Default|CallWSonHealthChanged 0.0 false)))
    (else
      (goto _label))))

(fn RunTime-IsActorAlive?
  (params (Actor%20Current%20Health :type Float%20%28double-precision%29))
  (if (>= Actor%20Current%20Health 3.0)
    (Variables|Default|SetIsAlive? true)
    (else
      (Variables|Default|SetIsAlive? false)))
  (return (Variables|Default|GetIsAlive?)))

(fn RunTime-HealthCalculation
  (params (InChangingHealth :type Float%20%28double-precision%29) (Medkit%20or%20Damage :type E_HealthChange%20Enum :default "NewEnumerator0"))
  (bind _maxhealth (Variables|Default|GetMaxHealth))
  (bind _maxhealth_2 (Variables|Default|GetMaxHealth))
  (Variables|Default|SetInChangingHealth InChangingHealth)
  (Variables|Default|SetMedkit%20or%20Damage Medkit%20or%20Damage)
  (switch Utilities|FlowControl|Switch|SwitchonE_HealthChange Medkit%20or%20Damage
    (:NewEnumerator0
      ;[1 0.7876 0.5244] Damage ( Decress HP )
      (bind _output_get (Variables|Default|SetHealth (Math|Float|Clamp(Float) (- (Variables|Default|GetHealth) (Variables|Default|GetInChangingHealth)) 0.0 _maxhealth_2)))
      (bind _healthprecent (CallFunction|Extra-HealthValuetoPercent _output_get _maxhealth_2))
      (return _healthprecent _output_get))
    (:NewEnumerator1
      ;[1 0.7876 0.5244] Medkit ( Incress HP )
      (bind _output_get_2 (Variables|Default|SetHealth (Math|Float|Clamp(Float) (+ (Variables|Default|GetHealth) (Variables|Default|GetInChangingHealth)) 0.0 _maxhealth)))
      (bind _healthprecent_2 (CallFunction|Extra-HealthValuetoPercent _output_get_2 _maxhealth))
      (return _healthprecent_2 _output_get_2))))

(fn Extra-CalculateDamage
  (params (Damage :type Float%20%28double-precision%29))
  (bind _output_get (LocalVariables|SetInDamage (Math|Conversions|ToFloat(Integer) (Math|Float|Round Damage))))
  (return _output_get))

(fn Extra-HealthValuetoPercent
  (params (HealthFloat :type Float%20%28double-precision%29) (MaxHealthFloat :type Float%20%28double-precision%29))
  (return 0.0))