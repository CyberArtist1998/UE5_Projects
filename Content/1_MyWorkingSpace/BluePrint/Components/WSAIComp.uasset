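; WSAIComp is an AI component for enemy behavior tree and blackboard setup, though that setup is currently disconnected.
; BeginPlay calls an empty Execute event; the unwired chain would cache the owner's AIC_EnemyAI, run the behavior tree, and seed the player target and behavior type.
; SetAIState writes the State blackboard key through that cached controller, which only the unwired chain assigns.
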(event Custom|Execute)

(event EventBeginPlay
  (CallFunction|Execute))

(fn SetAIState
  (params (State :type WSAiStateEnum%20Enum :default "NewEnumerator4"))
  (AI|Components|Blackboard|SetValueasEnum (AI|GetBlackboard (Variables|Default|GetAs%20AIC%20Enemy%20AI)) (Utilities|Name|MakeLiteralName "State") State))