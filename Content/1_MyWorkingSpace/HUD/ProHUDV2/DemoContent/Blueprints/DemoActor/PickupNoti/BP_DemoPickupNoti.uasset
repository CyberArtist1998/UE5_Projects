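; Demo actor for ProHUD V2 that pushes a pickup notification to the HUD manager when a ThirdPersonCharacter overlaps its box.
; Each notification uses the configured info and a tag with a random integer suffix, so repeated overlaps generally get different tags.
; The construction script mirrors the notification's icon on a billboard through a dynamic material with texture, color and emissive power, sized by a variable.
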(event OnComponentBeginOverlap(Box)
  (params (OverlappedComponent :type Primitive%20Component%20Object%20Reference) (OtherActor :type Actor%20Object%20Reference) (OtherComp :type Primitive%20Component%20Object%20Reference) (OtherBodyIndex :type Integer) (bFromSweep :type Boolean) (SweepResult :type Hit%20Result%20Structure%20%28by%20ref%29))
  (Utilities|Casting|CastToThirdPersonCharacter OtherActor)
  (Default|AddPickupNotification (CallFunction|GetHUDManager) (Utilities|String|Append (Variables|Default|GetTag) (Utilities|String|ToString(Integer) (Math|Random|RandomIntegerinRange 0 1024))) (Variables|Default|GetNotificationInfo)))

(event Custom|UpdateActor
  (bind _notificationinfo (Variables|Default|GetNotificationInfo))
  (bind (_icontexture _transform _iconcolor) (Utilities|Struct|BreakS_IconInfo2 (.iconinfo _notificationinfo)))
  (|CreateDynamicMaterialForBillboard_2_2)
  (|SetMaterialTexture_2_2 (.AsTexture (Utilities|Casting|CastToTexture _icontexture)))
  (|SetMaterialColor_2_2 _iconcolor)
  (|SetMaterialEmissive_2_2 (Variables|Default|GetEmissivePower))
  (|FinishMaterial_2_2))

(fn ConstructionScript
  (CallFunction|UpdateActor))