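; Function library for ProHUDV2 that supplies shared style and settings for the HUD's compass, minimap, markers and mission displays.
; Getters search for the first WB_HUD_Container widget on each call and read its properties, mostly with built-in fallbacks.
; Base, contrast and font colors also require the color stylesheet toggle.
; Helpers fetch player 0's HUD manager, read BP_CardinalDirection from the level, and apply stylesheet colors to unchanged icon colors.
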(fn GetHUDContainer
  (bind _foundwidgets (Widget|GetAllWidgetsOfClass 0 "/Game/1_MyWorkingSpace/HUD/ProHUDV2/Widgets/Content/WB_HUD_Container.WB_HUD_Container_C" false))
  (Utilities|IsValid (Utilities|Array|Get(acopy) _foundwidgets)
    (:Is%20Valid
      (return true (Utilities|Array|Get(acopy) _foundwidgets)))
    (:Is%20Not%20Valid
      (return false 0))))

(fn GetBaseColor1
  (bind (_returnvalue _hud_container) (References|GetHUDContainer))
  (if (and (Stylesheet|GetUseColorStylesheet) _returnvalue)
    (return (Variables|/Game/1_MyWorkingSpace/HUD/ProHUDV2/Widgets/Content/WB_HUD_Container.WB_HUD_Container_C|GetBaseColor1 _hud_container))
    (else
      (return "(R=1.000000,G=1.000000,B=1.000000,A=0.700000)"))))

(fn GetBaseColor2
  (bind (_returnvalue _hud_container) (References|GetHUDContainer))
  (if (and (Stylesheet|GetUseColorStylesheet) _returnvalue)
    (return (Variables|/Game/1_MyWorkingSpace/HUD/ProHUDV2/Widgets/Content/WB_HUD_Container.WB_HUD_Container_C|GetBaseColor2 _hud_container))
    (else
      (return "(R=1.000000,G=1.000000,B=1.000000,A=0.800000)"))))

(fn GetContrastColor1
  (bind (_returnvalue _hud_container) (References|GetHUDContainer))
  (if (and (Stylesheet|GetUseColorStylesheet) _returnvalue)
    (return (Variables|/Game/1_MyWorkingSpace/HUD/ProHUDV2/Widgets/Content/WB_HUD_Container.WB_HUD_Container_C|GetContrastColor1 _hud_container))
    (else
      (return "(R=0.010417,G=0.010417,B=0.010417,A=0.800000)"))))

(fn GetContrastColor2
  (bind (_returnvalue _hud_container) (References|GetHUDContainer))
  (if (and (Stylesheet|GetUseColorStylesheet) _returnvalue)
    (return (Variables|/Game/1_MyWorkingSpace/HUD/ProHUDV2/Widgets/Content/WB_HUD_Container.WB_HUD_Container_C|GetContrastColor2 _hud_container))
    (else
      (return "(R=0.010417,G=0.010417,B=0.010417,A=1.000000)"))))

(fn GetHeadlineFontInfo
  (bind (_returnvalue _hud_container) (References|GetHUDContainer))
  (if _returnvalue
    (return (Variables|/Game/1_MyWorkingSpace/HUD/ProHUDV2/Widgets/Content/WB_HUD_Container.WB_HUD_Container_C|GetHeadlineFont _hud_container))
    (else
      (return (Utilities|Struct|MakeSlateFontInfo "/Game/1_MyWorkingSpace/HUD/ProHUDV2/Fonts/F_Roboto.F_Roboto" 0 "(OutlineSize=0,bMiteredCorners=False,bSeparateFillAlpha=False,bApplyOutlineToDropShadows=False,OutlineMaterial=None,OutlineColor=(R=0.000000,G=0.000000,B=0.000000,A=1.000000))" "Roboto_Bold" (Math|Conversions|ToFloat(Integer) (Class|KismetSystemLibrary|MakeLiteralInteger 18)))))))

(fn GetBodyFontInfo
  (bind (_returnvalue _hud_container) (References|GetHUDContainer))
  (if _returnvalue
    (return (Variables|/Game/1_MyWorkingSpace/HUD/ProHUDV2/Widgets/Content/WB_HUD_Container.WB_HUD_Container_C|GetBodyFont _hud_container))
    (else
      (return (Utilities|Struct|MakeSlateFontInfo "/Game/1_MyWorkingSpace/HUD/ProHUDV2/Fonts/F_Roboto.F_Roboto" 0 "(OutlineSize=0,bMiteredCorners=False,bSeparateFillAlpha=False,bApplyOutlineToDropShadows=False,OutlineMaterial=None,OutlineColor=(R=0.000000,G=0.000000,B=0.000000,A=1.000000))" "Roboto_Regular" (Math|Conversions|ToFloat(Integer) (Class|KismetSystemLibrary|MakeLiteralInteger 14)))))))

(fn GetMicroFontInfo
  (bind (_returnvalue _hud_container) (References|GetHUDContainer))
  (if _returnvalue
    (return (Variables|/Game/1_MyWorkingSpace/HUD/ProHUDV2/Widgets/Content/WB_HUD_Container.WB_HUD_Container_C|GetMicroFont _hud_container))
    (else
      (return (Utilities|Struct|MakeSlateFontInfo "/Game/1_MyWorkingSpace/HUD/ProHUDV2/Fonts/F_Roboto.F_Roboto" 0 "(OutlineSize=0,bMiteredCorners=False,bSeparateFillAlpha=False,bApplyOutlineToDropShadows=False,OutlineMaterial=None,OutlineColor=(R=0.000000,G=0.000000,B=0.000000,A=1.000000))" "Roboto_LightItalic" (Math|Conversions|ToFloat(Integer) (Class|KismetSystemLibrary|MakeLiteralInteger 10)))))))

(fn GetUseColorStylesheet
  (bind (_returnvalue _hud_container) (References|GetHUDContainer))
  (if _returnvalue
    (return (Variables|/Game/1_MyWorkingSpace/HUD/ProHUDV2/Widgets/Content/WB_HUD_Container.WB_HUD_Container_C|GetbUseColorStyleSheet _hud_container))
    (else
      (return false))))

(fn GetHUDManager
  (bind _aspro_hudv2 (Utilities|Casting|CastToProHUDV2 (HUD|GetHUD (Game|GetPlayerController 0)))
    (:then
      (return _aspro_hudv2))
    (:CastFailed
      (Development|PrintString 0 "Please add the ProHUDV2 as HUD class to your game mode." true true "(R=1.000000,G=0.129199,B=0.125000,A=1.000000)" 1e+01)
      (Development|PrintString 0 "HUD Manager is not Valid." true true "(R=1.000000,G=0.004799,B=0.000000,A=1.000000)" 1e+01)
      (return 0))))

(fn GetDebugMessages
  (bind (_returnvalue _hud_container) (References|GetHUDContainer))
  (if _returnvalue
    (return (Variables|/Game/1_MyWorkingSpace/HUD/ProHUDV2/Widgets/Content/WB_HUD_Container.WB_HUD_Container_C|GetbGetDebugMessages _hud_container))
    (else
      (return false))))

(fn GetDistanceUnit
  (bind (_returnvalue _hud_container) (References|GetHUDContainer))
  (if _returnvalue
    (return (Variables|/Game/1_MyWorkingSpace/HUD/ProHUDV2/Widgets/Content/WB_HUD_Container.WB_HUD_Container_C|GetDistanceUnit _hud_container))
    (else
      (return "NewEnumerator1"))))

(fn GetMicroFont2Info
  (bind (_returnvalue _hud_container) (References|GetHUDContainer))
  (if _returnvalue
    (return (Variables|/Game/1_MyWorkingSpace/HUD/ProHUDV2/Widgets/Content/WB_HUD_Container.WB_HUD_Container_C|GetMicroFont2 _hud_container))
    (else
      (return (Utilities|Struct|MakeSlateFontInfo "/Game/1_MyWorkingSpace/HUD/ProHUDV2/Fonts/F_Roboto.F_Roboto" 0 "(OutlineSize=0,bMiteredCorners=False,bSeparateFillAlpha=False,bApplyOutlineToDropShadows=False,OutlineMaterial=None,OutlineColor=(R=0.000000,G=0.000000,B=0.000000,A=1.000000))" "Roboto_Italic" (Math|Conversions|ToFloat(Integer) (Class|KismetSystemLibrary|MakeLiteralInteger 10)))))))

(fn GetDistanceStepsKM
  (bind (_returnvalue _hud_container) (References|GetHUDContainer))
  (if _returnvalue
    (return (Variables|/Game/1_MyWorkingSpace/HUD/ProHUDV2/Widgets/Content/WB_HUD_Container.WB_HUD_Container_C|GetDistanceSteps_KM _hud_container))
    (else
      (return 100))))

(fn GetDistanceStepsM
  (bind (_returnvalue _hud_container) (References|GetHUDContainer))
  (if _returnvalue
    (return (Variables|/Game/1_MyWorkingSpace/HUD/ProHUDV2/Widgets/Content/WB_HUD_Container.WB_HUD_Container_C|GetDistanceSteps_M _hud_container))
    (else
      (return 1))))

(fn GetDistanceStepsMi
  (bind (_returnvalue _hud_container) (References|GetHUDContainer))
  (if _returnvalue
    (return (Variables|/Game/1_MyWorkingSpace/HUD/ProHUDV2/Widgets/Content/WB_HUD_Container.WB_HUD_Container_C|GetDistanceSteps_Mi _hud_container))
    (else
      (return 100))))

(fn GetDistanceStepsYa
  (bind (_returnvalue _hud_container) (References|GetHUDContainer))
  (if _returnvalue
    (return (Variables|/Game/1_MyWorkingSpace/HUD/ProHUDV2/Widgets/Content/WB_HUD_Container.WB_HUD_Container_C|GetDistanceSteps_Ya _hud_container))
    (else
      (return 1))))

(fn GetFontColor1
  (bind (_returnvalue _hud_container) (References|GetHUDContainer))
  (if (and (Stylesheet|GetUseColorStylesheet) _returnvalue)
    (return (Variables|/Game/1_MyWorkingSpace/HUD/ProHUDV2/Widgets/Content/WB_HUD_Container.WB_HUD_Container_C|GetFontColor1 _hud_container))
    (else
      (return "(R=1.000000,G=1.000000,B=1.000000,A=1.000000)"))))

(fn GetFontColor2
  (bind (_returnvalue _hud_container) (References|GetHUDContainer))
  (if (and (Stylesheet|GetUseColorStylesheet) _returnvalue)
    (return (Variables|/Game/1_MyWorkingSpace/HUD/ProHUDV2/Widgets/Content/WB_HUD_Container.WB_HUD_Container_C|GetFontColor2 _hud_container))
    (else
      (return "(R=1.000000,G=1.000000,B=1.000000,A=0.600000)"))))

(fn GetCompassBlendMask
  (bind (_returnvalue _hud_container) (References|GetHUDContainer))
  (bind _compass_blendmask (Variables|/Game/1_MyWorkingSpace/HUD/ProHUDV2/Widgets/Content/WB_HUD_Container.WB_HUD_Container_C|GetCompass_BlendMask _hud_container))
  (if _returnvalue
    (Utilities|IsValid _compass_blendmask
      (:Is%20Valid
        (return _compass_blendmask))
      (:Is%20Not%20Valid
        _)))
  (return 0))

(fn GetCompassTexture
  (bind (_returnvalue _hud_container) (References|GetHUDContainer))
  (bind _compass_texture (Variables|/Game/1_MyWorkingSpace/HUD/ProHUDV2/Widgets/Content/WB_HUD_Container.WB_HUD_Container_C|GetCompass_Texture _hud_container))
  (if _returnvalue
    (Utilities|IsValid _compass_texture
      (:Is%20Valid
        (return _compass_texture))
      (:Is%20Not%20Valid
        _)))
  (return 0))

(fn GetCompassBackgroundOpacity
  (bind (_returnvalue _hud_container) (References|GetHUDContainer))
  (if _returnvalue
    (return (Variables|/Game/1_MyWorkingSpace/HUD/ProHUDV2/Widgets/Content/WB_HUD_Container.WB_HUD_Container_C|GetCompass_BackgroundOpacity _hud_container))
    (else
      (return 1.0))))

(fn GetCompassTint
  (bind (_returnvalue _hud_container) (References|GetHUDContainer))
  (if _returnvalue
    (return (Variables|/Game/1_MyWorkingSpace/HUD/ProHUDV2/Widgets/Content/WB_HUD_Container.WB_HUD_Container_C|GetCompass_Tint _hud_container))
    (else
      (return "(R=1.000000,G=1.000000,B=1.000000,A=1.000000)"))))

(fn GetPointerTexture
  (bind (_returnvalue _hud_container) (References|GetHUDContainer))
  (if _returnvalue
    (return (Variables|/Game/1_MyWorkingSpace/HUD/ProHUDV2/Widgets/Content/WB_HUD_Container.WB_HUD_Container_C|GetPointerTexture _hud_container))
    (else
      (return "/Game/1_MyWorkingSpace/HUD/ProHUDV2/Textures/Compass/Pointers/T_Crosshair_500x1000_v2.T_Crosshair_500x1000_v2"))))

(fn GetPointerScale
  (bind (_returnvalue _hud_container) (References|GetHUDContainer))
  (if _returnvalue
    (return (Variables|/Game/1_MyWorkingSpace/HUD/ProHUDV2/Widgets/Content/WB_HUD_Container.WB_HUD_Container_C|GetPointerScale _hud_container))
    (else
      (return 1.0))))

(fn GetPointerYTranslation
  (bind (_returnvalue _hud_container) (References|GetHUDContainer))
  (if _returnvalue
    (return (Variables|/Game/1_MyWorkingSpace/HUD/ProHUDV2/Widgets/Content/WB_HUD_Container.WB_HUD_Container_C|GetPointerY_Translation _hud_container))
    (else
      (return 0.0))))

(fn GetPointerTint
  (bind (_returnvalue _hud_container) (References|GetHUDContainer))
  (if _returnvalue
    (return (Variables|/Game/1_MyWorkingSpace/HUD/ProHUDV2/Widgets/Content/WB_HUD_Container.WB_HUD_Container_C|GetPointerTint _hud_container))
    (else
      (return "(R=1.000000,G=1.000000,B=1.000000,A=1.000000)"))))

(fn GetMarkerYTranslation
  (bind (_returnvalue _hud_container) (References|GetHUDContainer))
  (if _returnvalue
    (return (Variables|/Game/1_MyWorkingSpace/HUD/ProHUDV2/Widgets/Content/WB_HUD_Container.WB_HUD_Container_C|GetMarkerY_Translation _hud_container))
    (else
      (return 0.0))))

(fn GetMarkerPrecision
  (bind (_returnvalue _hud_container) (References|GetHUDContainer))
  (if _returnvalue
    (return (Variables|/Game/1_MyWorkingSpace/HUD/ProHUDV2/Widgets/Content/WB_HUD_Container.WB_HUD_Container_C|GetMarkerPrecision _hud_container))
    (else
      (return 1.0))))

(fn GetCompassBackgroundTexture
  (bind (_returnvalue _hud_container) (References|GetHUDContainer))
  (if _returnvalue
    (return (Variables|/Game/1_MyWorkingSpace/HUD/ProHUDV2/Widgets/Content/WB_HUD_Container.WB_HUD_Container_C|GetCompass_BackgroundTexture _hud_container))
    (else
      (return "/Game/1_MyWorkingSpace/HUD/ProHUDV2/Textures/T_Mask_700x450.T_Mask_700x450"))))

(fn GetCompassBackgroundTransform
  (bind (_returnvalue _hud_container) (References|GetHUDContainer))
  (if _returnvalue
    (return (Variables|/Game/1_MyWorkingSpace/HUD/ProHUDV2/Widgets/Content/WB_HUD_Container.WB_HUD_Container_C|GetCompass_BackgroundTransform _hud_container))
    (else
      (return (Utilities|Struct|MakeWidgetTransform "(X=0.000000,Y=0.000000)")))))

(fn GetCompassBackgroundColor
  (bind (_returnvalue _hud_container) (References|GetHUDContainer))
  (if _returnvalue
    (return (Variables|/Game/1_MyWorkingSpace/HUD/ProHUDV2/Widgets/Content/WB_HUD_Container.WB_HUD_Container_C|GetCompass_BackgroundColor _hud_container))
    (else
      (return ""))))

(fn GetCompassOrientation
  (bind (_returnvalue _hud_container) (References|GetHUDContainer))
  (if _returnvalue
    (return (Variables|/Game/1_MyWorkingSpace/HUD/ProHUDV2/Widgets/Content/WB_HUD_Container.WB_HUD_Container_C|GetCompass_Direction _hud_container))
    (else
      (return 0.0))))

(fn GetMinimapSize
  (bind (_returnvalue _hud_container) (References|GetHUDContainer))
  (if _returnvalue
    (return (Variables|/Game/1_MyWorkingSpace/HUD/ProHUDV2/Widgets/Content/WB_HUD_Container.WB_HUD_Container_C|GetMinimap_Size _hud_container))
    (else
      (return 256.0))))

(fn GetMinimapMarkerMinMaxScale
  (bind (_returnvalue _hud_container) (References|GetHUDContainer))
  (bind _minimapmarker_minmaxscale (Variables|/Game/1_MyWorkingSpace/HUD/ProHUDV2/Widgets/Content/WB_HUD_Container.WB_HUD_Container_C|GetMinimapMarker_MinMaxScale _hud_container))
  (if _returnvalue
    (Development|PrintString 0 (Utilities|String|ToString(Vector2d) _minimapmarker_minmaxscale))
    (return _minimapmarker_minmaxscale)
    (else
      (return "(X=0.500000,Y=1.000000)"))))

(fn GetMinimapZoomInterpSpeed
  (bind (_returnvalue _hud_container) (References|GetHUDContainer))
  (if _returnvalue
    (return (Variables|/Game/1_MyWorkingSpace/HUD/ProHUDV2/Widgets/Content/WB_HUD_Container.WB_HUD_Container_C|GetMinimap_ZoomInterpSpeed _hud_container))
    (else
      (return 1.0))))

(fn GetMinimapPointerSize
  (bind (_returnvalue _hud_container) (References|GetHUDContainer))
  (if _returnvalue
    (return (Variables|/Game/1_MyWorkingSpace/HUD/ProHUDV2/Widgets/Content/WB_HUD_Container.WB_HUD_Container_C|GetMinimap_PointerSize _hud_container))
    (else
      (return 32.0))))

(fn GetMinimapPointerIcon
  (bind (_returnvalue _hud_container) (References|GetHUDContainer))
  (if _returnvalue
    (return (Variables|/Game/1_MyWorkingSpace/HUD/ProHUDV2/Widgets/Content/WB_HUD_Container.WB_HUD_Container_C|GetMinimap_PointerIcon _hud_container))
    (else
      (return "/Game/1_MyWorkingSpace/HUD/ProHUDV2/Textures/Minimap/T_Pointer1_64x64.T_Pointer1_64x64"))))

(fn GetMinimapPointerColor
  (bind (_returnvalue _hud_container) (References|GetHUDContainer))
  (if _returnvalue
    (return (Variables|/Game/1_MyWorkingSpace/HUD/ProHUDV2/Widgets/Content/WB_HUD_Container.WB_HUD_Container_C|GetMinimap_PointerColor _hud_container))
    (else
      (return "(R=1.000000,G=1.000000,B=1.000000,A=1.000000)"))))

(fn GetMinimapScalePointerwithZoom
  (bind (_returnvalue _hud_container) (References|GetHUDContainer))
  (if _returnvalue
    (return (Variables|/Game/1_MyWorkingSpace/HUD/ProHUDV2/Widgets/Content/WB_HUD_Container.WB_HUD_Container_C|GetbMinimap_ScalePointerWithZoom _hud_container))
    (else
      (return false))))

(fn GetMinimapPointerScaleMinMax
  (bind (_returnvalue _hud_container) (References|GetHUDContainer))
  (if _returnvalue
    (return (Variables|/Game/1_MyWorkingSpace/HUD/ProHUDV2/Widgets/Content/WB_HUD_Container.WB_HUD_Container_C|GetMinimap_PointerMinMax_Scale _hud_container))
    (else
      (return "(X=0.500000,Y=1.000000)"))))

(fn GetMinimapRotateMapwithPlayer
  (bind (_returnvalue _hud_container) (References|GetHUDContainer))
  (if _returnvalue
    (return (Variables|/Game/1_MyWorkingSpace/HUD/ProHUDV2/Widgets/Content/WB_HUD_Container.WB_HUD_Container_C|GetbRotateMinimapWithPlayer _hud_container))
    (else
      (return false))))

(fn GetCardinalDirection
  (bind _outactors (Actor|GetAllActorsOfClass 0 "/Game/1_MyWorkingSpace/HUD/ProHUDV2/Blueprints/Minimap/BP_CardinalDirection.BP_CardinalDirection_C"))
  (if (Utilities|Array|IsValidIndex _outactors)
    (Utilities|IsValid (Utilities|Array|Get(acopy) _outactors)
      (:Is%20Valid
        (return (Default|GetDirection (Utilities|Array|Get(acopy) _outactors))))
      (:Is%20Not%20Valid
        _)))
  (CallFunction|DebugPrint "No Cardinal Direction found." "Please add actor \"BP_Cardinal_Direction\" into your level.")
  (return -90))

(fn GetIsFirstPerson
  (bind (_returnvalue _hud_container) (References|GetHUDContainer))
  (if _returnvalue
    (return (Variables|/Game/1_MyWorkingSpace/HUD/ProHUDV2/Widgets/Content/WB_HUD_Container.WB_HUD_Container_C|GetbIsFirstPerson _hud_container))
    (else
      (return false))))

(fn GetMinimapTint
  (bind (_returnvalue _hud_container) (References|GetHUDContainer))
  (if _returnvalue
    (return (Variables|/Game/1_MyWorkingSpace/HUD/ProHUDV2/Widgets/Content/WB_HUD_Container.WB_HUD_Container_C|GetMinimapTint _hud_container))
    (else
      (return "(R=1.000000,G=1.000000,B=1.000000,A=1.000000)"))))

(fn GetMinimapMask
  (bind (_returnvalue _hud_container) (References|GetHUDContainer))
  (if _returnvalue
    (return (Variables|/Game/1_MyWorkingSpace/HUD/ProHUDV2/Widgets/Content/WB_HUD_Container.WB_HUD_Container_C|GetMinimapBlendMask _hud_container))
    (else
      (return "/Game/1_MyWorkingSpace/HUD/ProHUDV2/Textures/Minimap/T_MinimapMask1_256x256.T_MinimapMask1_256x256"))))

(fn GetDistantMarkerArrowIcon
  (bind (_returnvalue _hud_container) (References|GetHUDContainer))
  (if _returnvalue
    (return (Variables|/Game/1_MyWorkingSpace/HUD/ProHUDV2/Widgets/Content/WB_HUD_Container.WB_HUD_Container_C|GetDistantMarkerArrow _hud_container))
    (else
      (return "/Game/1_MyWorkingSpace/HUD/ProHUDV2/Textures/Minimap/T_Pointer1_64x64.T_Pointer1_64x64"))))

(fn GetMinimapFrame
  (bind (_returnvalue _hud_container) (References|GetHUDContainer))
  (if _returnvalue
    (return (Variables|/Game/1_MyWorkingSpace/HUD/ProHUDV2/Widgets/Content/WB_HUD_Container.WB_HUD_Container_C|GetMinimapFrame _hud_container))
    (else
      (return 0))))

(fn GetMinimapFrameTint
  (bind (_returnvalue _hud_container) (References|GetHUDContainer))
  (if _returnvalue
    (return (Variables|/Game/1_MyWorkingSpace/HUD/ProHUDV2/Widgets/Content/WB_HUD_Container.WB_HUD_Container_C|GetMinimapFrameTint _hud_container))
    (else
      (return "(R=1.000000,G=1.000000,B=1.000000,A=1.000000)"))))

(fn GetMinimapFrameScale
  (bind (_returnvalue _hud_container) (References|GetHUDContainer))
  (if _returnvalue
    (return (Variables|/Game/1_MyWorkingSpace/HUD/ProHUDV2/Widgets/Content/WB_HUD_Container.WB_HUD_Container_C|GetMinimapFrameScale _hud_container))
    (else
      (return ""))))

(fn GetMinimapScaleDistantMarkerwithZoom
  (bind (_returnvalue _hud_container) (References|GetHUDContainer))
  (if _returnvalue
    (return (Variables|/Game/1_MyWorkingSpace/HUD/ProHUDV2/Widgets/Content/WB_HUD_Container.WB_HUD_Container_C|GetbScaleDistantMarkerWithZoom _hud_container))
    (else
      (return false))))

(fn GetMinimapDistantMarkerMinMaxScale
  (bind (_returnvalue _hud_container) (References|GetHUDContainer))
  (if _returnvalue
    (return (Variables|/Game/1_MyWorkingSpace/HUD/ProHUDV2/Widgets/Content/WB_HUD_Container.WB_HUD_Container_C|GetMinimapDistantMarker_MinMaxScale _hud_container))
    (else
      (return "(X=1.000000,Y=1.000000)"))))

(fn GetVelocitySensitivity
  (bind (_returnvalue _hud_container) (References|GetHUDContainer))
  (if _returnvalue
    (return (Variables|/Game/1_MyWorkingSpace/HUD/ProHUDV2/Widgets/Content/WB_HUD_Container.WB_HUD_Container_C|GetVelocitySensitivity _hud_container))
    (else
      (return 0.0))))

(fn GetSensitivityInterpSpeed
  (bind (_returnvalue _hud_container) (References|GetHUDContainer))
  (if _returnvalue
    (return (Variables|/Game/1_MyWorkingSpace/HUD/ProHUDV2/Widgets/Content/WB_HUD_Container.WB_HUD_Container_C|GetSensitivityInterpSpeed _hud_container))
    (else
      (return 4.0))))

(fn GetCMarkerPingPlaybackSpeed
  (bind (_returnvalue _hud_container) (References|GetHUDContainer))
  (if _returnvalue
    (return (Variables|/Game/1_MyWorkingSpace/HUD/ProHUDV2/Widgets/Content/WB_HUD_Container.WB_HUD_Container_C|GetCMarker_PingPlaybackSpeed _hud_container))
    (else
      (return 3.0))))

(fn GetCMarkerPingDelay
  (bind (_returnvalue _hud_container) (References|GetHUDContainer))
  (if _returnvalue
    (return (Variables|/Game/1_MyWorkingSpace/HUD/ProHUDV2/Widgets/Content/WB_HUD_Container.WB_HUD_Container_C|GetCMarker_PingDelay _hud_container))
    (else
      (return 2.0))))

(fn GetMissionNotificationInfo
  (bind (_returnvalue _hud_container) (References|GetHUDContainer))
  (if _returnvalue
    (return (Variables|/Game/1_MyWorkingSpace/HUD/ProHUDV2/Widgets/Content/WB_HUD_Container.WB_HUD_Container_C|GetMissionNotificationInfo _hud_container))
    (else
      (return (Utilities|Struct|MakeS_MissionNotiBaseInfo 256.0 "(UseManualFontInfo_14_951431AC44031EEE99FEF1A339E21EA7=False,FontInfo_11_34A088E64B813A23F8385280F346B6C3=(FontObject=None,FontMaterial=None,OutlineSettings=(OutlineSize=0,bMiteredCorners=False,bSeparateFillAlpha=False,bApplyOutlineToDropShadows=False,OutlineMaterial=None,OutlineColor=(R=0.000000,G=0.000000,B=0.000000,A=1.000000)),TypefaceFontName=\"\",Size=24.000000,LetterSpacing=0,SkewAmount=0.000000,bForceMonospaced=False,bMaterialIsStencil=False,MonospacedWidth=1.000000),Scale_5_0E74308D459AEBE0552A83B12AC2CFC5=1.000000,ColorAndOpacity_8_453565FB47559D18C939A3B22216E9F0=(R=0.000000,G=0.000000,B=0.000000,A=0.000000))")))))

(fn GetMissionTasksInfo
  (bind (_returnvalue _hud_container) (References|GetHUDContainer))
  (if _returnvalue
    (return (Variables|/Game/1_MyWorkingSpace/HUD/ProHUDV2/Widgets/Content/WB_HUD_Container.WB_HUD_Container_C|GetMissionTasksInfo _hud_container))
    (else
      (return (Utilities|Struct|MakeS_TaskBaseInfo 2e+01 0.0)))))

(fn GetBodyFont2Info
  (bind (_returnvalue _hud_container) (References|GetHUDContainer))
  (if _returnvalue
    (return (Variables|/Game/1_MyWorkingSpace/HUD/ProHUDV2/Widgets/Content/WB_HUD_Container.WB_HUD_Container_C|GetBodyFont2 _hud_container))
    (else
      (return (Utilities|Struct|MakeSlateFontInfo "/Game/1_MyWorkingSpace/HUD/ProHUDV2/Fonts/F_Roboto.F_Roboto" 0 "(OutlineSize=0,bMiteredCorners=False,bSeparateFillAlpha=False,bApplyOutlineToDropShadows=False,OutlineMaterial=None,OutlineColor=(R=0.000000,G=0.000000,B=0.000000,A=1.000000))" "Roboto_Bold" (Math|Conversions|ToFloat(Integer) (Class|KismetSystemLibrary|MakeLiteralInteger 14)))))))

(fn FindIconColor
  (params (S_IconInfo :type S%20Icon%20Info%20Structure%20%28by%20ref%29) (StylesheetColor :type Linear%20Color%20Structure))
  (bind (_icontexture _size _iconcolor _highlightcolor) (Utilities|Struct|BreakS_IconInfo S_IconInfo))
  (return (Utilities|Struct|MakeS_IconInfo _icontexture _size (select (CallFunction|HasColorChanged _iconcolor) _iconcolor StylesheetColor) _highlightcolor)))

(fn FindIcon2Color
  (params (S_IconInfo2 :type S%20Icon%20Info%202%20Structure%20%28by%20ref%29) (StylesheetColor :type Linear%20Color%20Structure))
  (bind (_icontexture _transform _iconcolor) (Utilities|Struct|BreakS_IconInfo2 S_IconInfo2))
  (return (Utilities|Struct|MakeS_IconInfo2 _icontexture _transform (select (CallFunction|HasColorChanged _iconcolor) _iconcolor StylesheetColor))))